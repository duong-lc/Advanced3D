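; TargetManager is a puzzle controller that links a set of targets to a door and a reward pad.
; It binds to each target's enabled and disabled events to keep a count, opening the door when all are enabled and closing it when any drops out.
; While the condition holds, the destination pad's event spawns a BP_PickUpOrbitalStrike just above the pad, only once.
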(event `self.ReceiveBeginPlay`
  (add `/Game/Blueprint/TargetManager/DestinationPad.EventDestinationPad` (`self.pad`) (`|CreateDelegate` :!event `OnDestinationPad`))
  (for _array_element (`self.Targets`)
    (add `/Game/Blueprint/TargetManager/Target.EventTargetEnabled` _array_element (`|CreateDelegate` :!event `OnTargetEnabled`))
    (add `/Game/Blueprint/TargetManager/Target.EventTargetDisabled` _array_element (`|CreateDelegate` :!event `OnTargetDisabled`))))

(event `OnTargetEnabled`
  (bind _result (`/Engine/EditorBlueprintResources/StandardMacros.IncrementInt` (`self.numEnabled`))
    (:`  `
      (if (== _result (`KismetArrayLibrary.Array_Length` (`self.Targets`)))
        (set `self.conditionMet` true)
        (`/Game/Blueprint/TargetManager/Door.Open Door` (`self.Door`))))))

(event `OnTargetDisabled`
  (`/Engine/EditorBlueprintResources/StandardMacros.DecrementInt` (`self.numEnabled`)
    (:`  `
      (if (`self.conditionMet`)
        (set `self.conditionMet` false)
        (`/Game/Blueprint/TargetManager/Door.Close Door` (`self.Door`))))))

(event `OnDestinationPad`
  (bind (_returnvalue_location _returnvalue_rotation _returnvalue_scale) (`KismetMathLibrary.BreakTransform` (`self.GetTransform` (`self.pad`))))
  (if (`self.conditionMet`)
    (if (not (`self.spawned`))
      (`KismetSystemLibrary.PrintString` "asdadsa")
      (`|SpawnActorFromClass` "/Game/Blueprint/WeaponPickUp/BP_PickUpOrbitalStrike.BP_PickUpOrbitalStrike_C" (`KismetMathLibrary.MakeTransform` (+ _returnvalue_location (0.0 0.0 10.0)) _returnvalue_rotation _returnvalue_scale) "Undefined" "OverrideRootScale" null null)
      (set `self.spawned` true))))

(fn `UserConstructionScript`)