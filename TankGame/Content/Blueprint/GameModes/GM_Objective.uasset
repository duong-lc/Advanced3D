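; GM_Objective is a game mode Blueprint that overrides FindPlayerStart to choose spawn points from BP_TankPlayerStart actors.
; It adds every such start in the level to NoTeamPlayerStartArray, then returns a random entry when a random entry's IsOverlap check is true.
; The check and the return each call Random, so they can pick different starts, and no fallback handles a false result.
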(fn `FindPlayerStart`
  (params (Player :type "Controller Object Reference") (IncomingName :type String))
  (returns (ReturnValue :type "Actor Object Reference"))
  (bind _outitem (`KismetArrayLibrary.Array_Random` (`self.No Team Player Start Array`)))
  (bind _outactors (`GameplayStatics.GetAllActorsOfClass` "/Game/Blueprint/Teams/BP_TankPlayerStart.BP_TankPlayerStart_C"))
  (for _array_element _outactors
    (`KismetArrayLibrary.Array_AddUnique` (`self.No Team Player Start Array`) _array_element))
  (if (`/Game/Blueprint/Teams/BP_TankPlayerStart.IsOverlap` _outitem)
    (return _outitem)))

(fn `UserConstructionScript`
  (`parent.UserConstructionScript`))