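; GM_Zombie is the game mode for zombie mode, setting up in-game UI for player controllers on BeginPlay.
; SetUpUI loops over the controllers, creates the zombie-mode widget for each valid one, cross-links it with PC_ZombieMode, hands it to that player's tank and shows the mouse cursor.
; A helper, GetPlayerControllerIndex, finds which controller index owns a given pawn and reports whether one was found.
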(event `self.ReceiveBeginPlay`
  (`self.SetUpUI`))

(fn `GetPlayerControllerIndex`
  (params (Pawn :type "Pawn Object Reference"))
  (returns (Index :type Integer) (`is PC found` :type Boolean))
  (locals (pawnToCompare :type "Pawn Object Reference") (ControllerIndex :type Integer) (isPCFound :type Boolean :default false))
  (set `local.pawnToCompare` Pawn)
  (set `local.isPCFound` false)
  (for _index (range (`GameplayStatics.GetNumPlayerControllers`))
    (bind _aspc_zombie_mode (cast `/Game/Blueprint/PlayerControllers/PC_ZombieMode` (`GameplayStatics.GetPlayerController` _index)))
    (bind _aspc_zombie_mode_2 (cast `/Game/Blueprint/PlayerControllers/PC_ZombieMode` (`Pawn.GetController` (`local.pawnToCompare`))))
    (if (== _aspc_zombie_mode_2 _aspc_zombie_mode)
      (set `local.ControllerIndex` _index)
      (set `local.isPCFound` true)
      (break)))
  (return (`local.ControllerIndex`) (`local.isPCFound`)))

(fn `SetUpUI`
  (locals (`Local UI Instance` :type "/Game/Blueprint/HUD/UI_InGame_ZombieMode Object Reference"))
  (for _index (range (`GameplayStatics.GetNumPlayerControllers`))
    (bind _returnvalue (`GameplayStatics.GetPlayerController` _index))
    (`/Engine/EditorBlueprintResources/StandardMacros.IsValid` _returnvalue
      (:`Is Valid`
        (`|ExecutionSequence`
          (:`then_0`
            (bind _returnvalue_2 (`|CreateWidget` (`self.UI_InGame_Player`)))
            (bind _output_get (set `local.Local UI Instance` _returnvalue_2))
            (`UserWidget.AddToViewport` _output_get 0))
          (:`then_1`
            (bind _aspc_zombie_mode (cast `/Game/Blueprint/PlayerControllers/PC_ZombieMode` _returnvalue))
            (set `/Game/Blueprint/PlayerControllers/PC_ZombieMode.InGameUI` (`local.Local UI Instance`) _aspc_zombie_mode)
            (set `/Game/Blueprint/HUD/UI_InGame_ZombieMode.PC_Inst` _aspc_zombie_mode (`local.Local UI Instance`))
            (set `/Game/Blueprint/TankPawns/PlayerZombiePawns/P_TankZombieMode.UI_InGame` (`local.Local UI Instance`) (`/Game/Blueprint/PlayerControllers/PC_ZombieMode.playerTank` _aspc_zombie_mode))
            (set `PlayerController.bShowMouseCursor` true _aspc_zombie_mode)))))))

(fn `UserConstructionScript`
  (set `self.UI_InGame_Player` "/Game/Blueprint/HUD/UI_InGame_ZombieMode.UI_InGame_ZombieMode_C"))