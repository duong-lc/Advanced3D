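; Game mode for a timed Red vs Blue tank capture-objective match with local players and AI filling remaining slots.
; On BeginPlay it caches the objective and waypoints, spawns player tanks with HUDs and team-colored cursors, then teleports AI to alternating team spawns, falling back to the other team.
; GetRandomWayPoint sends AI toward the objective, or toward enemy waypoints when their team holds it.
; A ready-up overlay pauses play; win and lose handlers only print.
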(event `self.ReceiveBeginPlay`
  (`KismetSystemLibrary.PrintString` "Spawning Player OBJ")
  (set `self.Timer` 120)
  (set `self.isGameTimeOrientated` true)
  (`parent.ReceiveBeginPlay`)
  (`self.SetupObjectiveGMRefs`)
  (`self.SetUpPlayerSpawnRefs`)
  (`|ExecutionSequence`
    (:`then_0`
      (for _array_element (`self.All Players`)
        (`KismetSystemLibrary.PrintString` "Spawning Player OBJ")
        (`self.Spawn Player` _array_element)))
    (:`then_1`
      (`self.Spawn All AI`))
    (:`then_2`
      (bind _returnvalue (`|CreateWidget` (`self.UIEnd Screen Class`)))
      (set `self.UIEndScreenRef` _returnvalue))))

(event `Win State`
  (params (Winner :type "Pawn Object Reference"))
  (`KismetSystemLibrary.PrintString` (`KismetSystemLibrary.GetDisplayName` Winner)))

(event `Lose State`
  (`self.LoseState`))

(event `self.ReceiveTick`
  (params (DeltaSeconds :type "Float (single-precision)")))

(event `/Game/Blueprint/GameModes/GM_Multiplayer_Interface.OnReadyUpOff`
  (`Widget.RemoveFromParent` (`self.ReadyUpOverlayRef`))
  (`GameplayStatics.SetGamePaused` false))

(event `/Game/Blueprint/GameModes/GM_Multiplayer_Interface.OnReadyUpOn`
  (bind _readyupoverlayref (`self.ReadyUpOverlayRef`))
  (`UserWidget.AddToViewport` _readyupoverlayref 0)
  (`/Game/Blueprint/UI_AllGMReadyUpOverlay.OnDisplayReadyUp` _readyupoverlayref (+ (`self.localPlayersCount`) 2))
  (`GameplayStatics.SetGamePaused` true)
  (`/Game/Blueprint/UI_AllGMReadyUpOverlay.Player Ready Up On` (`self.ReadyUpOverlayRef`))
  (`/Game/Blueprint/UI_AllGMReadyUpOverlay.Player Ready Up Off` (`self.ReadyUpOverlayRef`)))

(event `/Game/Blueprint/GameModes/GM_Multiplayer_Interface.OnReadyUpInput`
  (params (ReadyState :type Boolean))
  (if ReadyState
    (`/Game/Blueprint/UI_AllGMReadyUpOverlay.Player Ready Up On` (`self.ReadyUpOverlayRef`))
    (else
      (`/Game/Blueprint/UI_AllGMReadyUpOverlay.Player Ready Up Off` (`self.ReadyUpOverlayRef`)))))

(fn `AddTotalPlayers`
  (locals (playerCountTemp :type Integer :default 0) (`is A` :type Boolean :default false))
  (if (> (`self.maxPlayerInGame`) 0)
    (bind _output_get (set `self.localPlayersCount` (- (`KismetStringLibrary.Conv_StringToInt` (`GameplayStatics.ParseOption` (`self.OptionsString`) "players")) 2)))
    (set `self.AIPlayerCount` (- (`self.maxPlayerInGame`) (`self.localPlayersCount`)))
    (for _index (range (+ _output_get 1))
      (if (!= (mod _index 2) 0)
        (bind _aspc_base (`self.AddLocalPlayer`))
        (`/Game/Blueprint/PlayerControllers/PC_Base.SetTeam` _aspc_base "NewEnumerator2")
        (else
          (bind _aspc_base_2 (`self.AddLocalPlayer`))
          (`/Game/Blueprint/PlayerControllers/PC_Base.SetTeam` _aspc_base_2 "NewEnumerator1"))))))

(fn `GetObjectiveRef`
  (returns (ObjectiveRef :type "/Game/Blueprint/CaptureObj/BP_Objective Object Reference"))
  (return (`self.ObjectiveRef`)))

(fn `GetRandomWayPoint`
  (params (`AI Team` :type "/Game/Blueprint/Teams/EnumTeams Enum" :default "NewEnumerator0"))
  (returns (WayPointRef :type "/Game/Blueprint/CaptureObj/AI_WayPoint Object Reference"))
  (bind _objectiveref (`self.GetObjectiveRef`))
  (switch `/Game/Blueprint/Teams/EnumTeams` `AI Team`
    (:`NewEnumerator0`
      (`KismetSystemLibrary.PrintString` "GM_OBJ: WHY IS IT NO TEAM"))
    (:`NewEnumerator1`
      (switch `/Game/Blueprint/CaptureObj/ObjectiveStatusEnum` (`/Game/Blueprint/CaptureObj/BP_Objective.ObjectiveStatus` _objectiveref)
        (:`NewEnumerator0`
          (return (`KismetArrayLibrary.Array_Random` (`self.BlueTeamAIWayPoint`))))
        (:`NewEnumerator1`
          _)
        (:`NewEnumerator2`
          _))
      (return (`KismetArrayLibrary.Array_Random` (`self.ObjAIWayPoint`))))
    (:`NewEnumerator2`
      (switch `/Game/Blueprint/CaptureObj/ObjectiveStatusEnum` (`/Game/Blueprint/CaptureObj/BP_Objective.ObjectiveStatus` _objectiveref)
        (:`NewEnumerator0`
          _)
        (:`NewEnumerator1`
          (return (`KismetArrayLibrary.Array_Random` (`self.RedTeamAIWayPoint`))))
        (:`NewEnumerator2`
          _))
      (return (`KismetArrayLibrary.Array_Random` (`self.ObjAIWayPoint`))))))

(fn `Initialize AI Pawn`
  (params (`Ai Controller` :type "/Game/Blueprint/EnemyMob/captureObjective/AIC_CaptureObjective Object Reference") (TeamToSpawn :type "/Game/Blueprint/Teams/EnumTeams Enum" :default "NewEnumerator0"))
  (returns (`Spawn Success?` :type Boolean))
  (bind (_spawntransform _spawnactor _isfound) (`self.Get AI Spawn Point` TeamToSpawn `Ai Controller`))
  (message `/Game/Blueprint/PlayerControllers/Interface_TeamPlayerController.SetTeam` `Ai Controller` TeamToSpawn)
  (if _isfound
    (`self.K2_SetActorTransform` (`Controller.K2_GetPawn` `Ai Controller`) _spawntransform false true)
    (bind _aic_ref (`/Game/Blueprint/Teams/BP_TankPlayerStart.Link Current AIC Ref` _spawnactor `Ai Controller`))
    (message `/Game/Blueprint/PlayerControllers/Interface_TeamPlayerController.SetPlayerStart` _aic_ref _spawnactor))
  (return _isfound))

(fn `LoseState`
  (`KismetSystemLibrary.PrintString` "Capture Objective Game mode ended" true true (struct :`R` 1.0 :`G` 0.009923 :`B` 0.03977 :`A` 1.0)))

(fn `SetupObjectiveGMRefs`
  (`|ExecutionSequence`
    (:`then_0`
      ;[1 1 1] Set Up Ref For Objective Point
      (bind _outactors (`GameplayStatics.GetAllActorsOfClass` "/Game/Blueprint/CaptureObj/BP_Objective.BP_Objective_C"))
      (if (> (`KismetArrayLibrary.Array_Length` _outactors) 1)
        (`KismetSystemLibrary.PrintString` "THERE SHOULDN'T BE MORE THAN 1 OBJECTIVE IN GM" true true (struct :`R` 1.0 :`B` 0.205922 :`A` 1.0))
        (else
          (set `self.ObjectiveRef` (`|GetArrayItem` _outactors)))))
    (:`then_1`
      (bind _outactors_2 (`GameplayStatics.GetAllActorsOfClass` "/Game/Blueprint/CaptureObj/AI_WayPoint.AI_WayPoint_C"))
      (for _array_element _outactors_2
        (switch `/Game/Blueprint/CaptureObj/AI_WayPointEnum` (`/Game/Blueprint/CaptureObj/AI_WayPoint.WayPointID` _array_element)
          (:`NewEnumerator0`
            (`KismetArrayLibrary.Array_AddUnique` (`self.ObjAIWayPoint`) _array_element))
          (:`NewEnumerator1`
            (`KismetArrayLibrary.Array_AddUnique` (`self.RedTeamAIWayPoint`) _array_element))
          (:`NewEnumerator2`
            (`KismetArrayLibrary.Array_AddUnique` (`self.BlueTeamAIWayPoint`) _array_element)))))))

(fn `SetUpUIMouseCursor`
  (params (Controller :type "Controller Object Reference"))
  (bind _ui_instance (`parent.SetUpUIMouseCursor` Controller))
  (bind _team (message `/Game/Blueprint/PlayerControllers/Interface_TeamPlayerController.GetTeam` (`/Game/Blueprint/PlayerControllers/UI_MouseCursor.PC inst` _ui_instance)))
  (switch `/Game/Blueprint/Teams/EnumTeams` _team
    (:`NewEnumerator1`
      (bind _mousecursor (`/Game/Blueprint/PlayerControllers/UI_MouseCursor.MouseCursor` _ui_instance))
      (`Image.SetColorAndOpacity` _mousecursor (struct :`R` 1.0 :`B` 0.13424 :`A` 1.0)))
    (:`NewEnumerator2`
      (`Image.SetColorAndOpacity` _mousecursor (struct :`G` 0.77537 :`B` 1.0 :`A` 1.0)))))

(fn `Spawn All AI`
  (for _ (range 1 (+ (- (`self.AIPlayerCount`) 2) 1))
    (bind _returnvalue (`|SpawnActorFromClass` "/Game/Blueprint/EnemyMob/captureObjective/P_AI_CaptureObjective.P_AI_CaptureObjective_C" (`KismetMathLibrary.MakeTransform` (0.0 0.0 110.0)) "AlwaysSpawn" "OverrideRootScale" null null))
    (`KismetSystemLibrary.PrintString` (`KismetSystemLibrary.GetDisplayName` _returnvalue))
    (bind _ai_controller (`/Game/Blueprint/EnemyMob/captureObjective/P_AI_CaptureObjective.Get AI Controller` _returnvalue))
    (`KismetArrayLibrary.Array_AddUnique` (`self.All AI Controllers`) _ai_controller))
  (for (_array_element _array_index) (`self.All AI Controllers`)
    (bind _asaic_capture_objective (cast `/Game/Blueprint/EnemyMob/captureObjective/AIC_CaptureObjective` _array_element))
    (if (== (mod _array_index 2) 0)
      (bind _spawn_success_ (`self.Initialize AI Pawn` _asaic_capture_objective "NewEnumerator2"))
      (if (not _spawn_success_)
        (`self.Initialize AI Pawn` _asaic_capture_objective "NewEnumerator1"))
      (else
        (bind _spawn_success__2 (`self.Initialize AI Pawn` _asaic_capture_objective "NewEnumerator1"))
        (if (not _spawn_success__2)
          (`self.Initialize AI Pawn` _asaic_capture_objective "NewEnumerator2"))))))

(fn `Spawn Player`
  (params (Controller :type "Controller Object Reference"))
  (locals (UI_Inst :type "/Game/Blueprint/CaptureObj/UI_InGameCaptureObj Object Reference"))
  (bind _aspc_capture_obj (cast `/Game/Blueprint/PlayerControllers/PC_CaptureObj` Controller))
  (bind _team (message `/Game/Blueprint/PlayerControllers/Interface_TeamPlayerController.GetTeam` Controller))
  (bind (_spawntransform _spawnactor _isfound) (`self.Get Player Spawn Point` _team _aspc_capture_obj))
  (if _isfound
    (bind _pcref (`/Game/Blueprint/Teams/BP_TankPlayerStart.Link Current PC Ref` _spawnactor _aspc_capture_obj))
    (set `/Game/Blueprint/PlayerControllers/PC_Base.CurrentSpawner` _spawnactor _pcref)
    (bind _returnvalue (`|SpawnActorFromClass` "/Game/Blueprint/TankPawns/CaptureObjectivePawns/P_TankObjective.P_TankObjective_C" _spawntransform "Undefined" "OverrideRootScale" null null))
    (bind _returnvalue_2 (`|CreateWidget` "/Game/Blueprint/CaptureObj/UI_InGameCaptureObj.UI_InGameCaptureObj_C" _aspc_capture_obj))
    (bind _output_get (set `local.UI_Inst` _returnvalue_2))
    (`/Game/Blueprint/CaptureObj/UI_InGameCaptureObj.SetUpRefs` _output_get _aspc_capture_obj)
    (`UserWidget.AddToPlayerScreen` _output_get 0)
    (`self.SetUpUIMouseCursor` _aspc_capture_obj)
    (message `/Game/Blueprint/PlayerControllers/PC_ObjectiveInterface.LinkUIRef` _aspc_capture_obj _output_get)
    (`KismetSystemLibrary.PrintString` "POSSESS OBJ PAWN")
    (`Controller.Possess` _aspc_capture_obj _returnvalue)
    (else
      (`KismetSystemLibrary.PrintString` "can't find spawner"))))

(fn `UserConstructionScript`)