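; Base game mode for a local multiplayer tank game, handling players, team spawns, match readiness and end conditions.
; BeginPlay creates extra local players from the "players" option, caches tank starts by team and optionally starts a loss countdown.
; Logins get cursor widgets, logouts leave the last player winning, and PC_Base ready flags gate match start and end.
; Team-based spawn helpers exist, but the spawn-all loop is unwired; win/lose only print.
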(event `self.ReceiveBeginPlay`
  (bind _returnvalue (- (`KismetStringLibrary.Conv_StringToInt` (`GameplayStatics.ParseOption` (`self.OptionsString`) "players")) 2))
  (if (>= _returnvalue -1)
    (for _ (range (+ _returnvalue 1))
      (`KismetSystemLibrary.PrintString` (`KismetStringLibrary.Conv_IntToString` _returnvalue))
      (`GameplayStatics.CreatePlayer` -1))
    (`|ExecutionSequence`
      (:`then_0`
        (`self.SetUpPlayerSpawnRefs`))
      (:`then_3`
        (if (`self.isGameTimeOrientated`)
          (bind _returnvalue_2 (`KismetSystemLibrary.K2_SetTimerDelegate` (delegate `TimerCountDown`) 1.0 true)))))))

(event `TimerCountDown`
  (`/Engine/EditorBlueprintResources/StandardMacros.DecrementInt` (`self.Timer`)
    (:`  `
      (if (<= (`self.Timer`) 0)
        (`self.Lose State`)
        (`KismetSystemLibrary.K2_ClearAndInvalidateTimerHandle` (stale `self.ReceiveBeginPlay` _returnvalue_2))))))

(event `Win State`
  (params (Winner :type "Pawn Object Reference"))
  (`KismetSystemLibrary.PrintString` (`KismetSystemLibrary.GetDisplayName` Winner)))

(event `Lose State`
  (`KismetSystemLibrary.PrintString` "Lose GM_BASe"))

(event `self.K2_PostLogin`
  (params (NewPlayer :type "PlayerController Object Reference"))
  (`KismetArrayLibrary.Array_AddUnique` (`self.Players`) NewPlayer)
  (`self.SetUpUIMouseCursor` NewPlayer))

(event `self.K2_OnLogout`
  (params (ExitingController :type "Controller Object Reference"))
  (`KismetArrayLibrary.Array_RemoveItem` (`self.Players`) ExitingController)
  (if (== (`KismetArrayLibrary.Array_Length` (`self.Players`)) 1)
    (`self.Win State` (`Controller.K2_GetPawn` (`|GetArrayItem` (`self.Players`))))))

(event `self.K2_OnSetMatchState`
  (params (NewState :type Name))
  (`KismetSystemLibrary.PrintString` (`KismetStringLibrary.Conv_NameToString` NewState))
  (`KismetSystemLibrary.PrintString` (`KismetStringLibrary.Conv_NameToString` (`self.GetMatchState`)))
  (switch `name` NewState))

(fn `FindPlayerStart`
  (params (Player :type "Controller Object Reference") (IncomingName :type String))
  (returns (ReturnValue :type "Actor Object Reference"))
  (bind _outitem (`KismetArrayLibrary.Array_Random` (`self.Blue Team Player Start Array`)))
  (bind _outitem_2 (`KismetArrayLibrary.Array_Random` (`self.No Team Player Start Array`)))
  (bind _outitem_3 (`KismetArrayLibrary.Array_Random` (`self.Red Team Player Start Array`)))
  (bind _outactors (`GameplayStatics.GetAllActorsOfClass` "/Game/Blueprint/Teams/BP_TankPlayerStart.BP_TankPlayerStart_C"))
  (for _array_element _outactors
    (switch `/Game/Blueprint/Teams/EnumTeams` (`/Game/Blueprint/Teams/BP_TankPlayerStart.Team` _array_element)
      (:`NewEnumerator0`
        (`KismetArrayLibrary.Array_AddUnique` (`self.No Team Player Start Array`) _array_element))
      (:`NewEnumerator1`
        (`KismetArrayLibrary.Array_AddUnique` (`self.Red Team Player Start Array`) _array_element))
      (:`NewEnumerator2`
        (`KismetArrayLibrary.Array_AddUnique` (`self.Blue Team Player Start Array`) _array_element))))
  (bind _team (message `/Game/Blueprint/PlayerControllers/Interface_TeamPlayerController.GetTeam` Player))
  (`KismetSystemLibrary.PrintString` (`|GetEnumeratorNameAsString` _team))
  (switch `/Game/Blueprint/Teams/EnumTeams` _team :!label _label
    (:`NewEnumerator0`
      (if (`/Game/Blueprint/Teams/BP_TankPlayerStart.IsOverlap` _outitem_2)
        (return _outitem_2)
        (else
          (goto _label))))
    (:`NewEnumerator1`
      (if (`/Game/Blueprint/Teams/BP_TankPlayerStart.IsOverlap` _outitem_3)
        (return _outitem_3)
        (else
          (goto _label))))
    (:`NewEnumerator2`
      (if (`/Game/Blueprint/Teams/BP_TankPlayerStart.IsOverlap` _outitem)
        (return _outitem)
        (else
          (goto _label))))))

(fn `ReadyToEndMatch`
  (returns (ReturnValue :type Boolean))
  (for _array_element (`self.Players`)
    (bind _aspc_base (cast `/Game/Blueprint/PlayerControllers/PC_Base` _array_element))
    (if (`/Game/Blueprint/PlayerControllers/PC_Base.isReady` _aspc_base)
      (return false)))
  (return true))

(fn `ReadyToStartMatch`
  (returns (ReturnValue :type Boolean))
  (for _array_element (`self.Players`)
    (bind _aspc_base (cast `/Game/Blueprint/PlayerControllers/PC_Base` _array_element))
    (if (not (`/Game/Blueprint/PlayerControllers/PC_Base.isReady` _aspc_base))
      (return false)))
  (return true))

(fn `SetUpPlayerSpawnRefs`
  (bind _outactors (`GameplayStatics.GetAllActorsOfClass` "/Game/Blueprint/Teams/BP_TankPlayerStart.BP_TankPlayerStart_C"))
  (for _array_element _outactors
    (switch `/Game/Blueprint/Teams/EnumTeams` (`/Game/Blueprint/Teams/BP_TankPlayerStart.Team` _array_element)
      (:`NewEnumerator0`
        (`KismetArrayLibrary.Array_AddUnique` (`self.No Team Player Start Array`) _array_element))
      (:`NewEnumerator1`
        (`KismetArrayLibrary.Array_AddUnique` (`self.Red Team Player Start Array`) _array_element))
      (:`NewEnumerator2`
        (`KismetArrayLibrary.Array_AddUnique` (`self.Blue Team Player Start Array`) _array_element)))))

(fn `SetUpUIMouseCursor`
  (params (Controller :type "Controller Object Reference"))
  (locals (`Local UI Instance` :type "/Game/Blueprint/PlayerControllers/UI_MouseCursor Object Reference"))
  (`/Engine/EditorBlueprintResources/StandardMacros.IsValid` Controller
    (:`Is Valid`
      (`|ExecutionSequence`
        (:`then_0`
          (bind _returnvalue (`|CreateWidget` (`self.UI_MouseCursor`)))
          (bind _output_get (set `local.Local UI Instance` _returnvalue))
          (`UserWidget.AddToViewport` _output_get 0))
        (:`then_1`
          (bind _aspc_base (cast `/Game/Blueprint/PlayerControllers/PC_Base` Controller))
          (set `/Game/Blueprint/PlayerControllers/PC_Base.CursorUI` (`local.Local UI Instance`) _aspc_base)
          (set `/Game/Blueprint/PlayerControllers/UI_MouseCursor.PC inst` _aspc_base (`local.Local UI Instance`)))))))

(fn `Spawn Player`
  (params (Controller :type "Controller Object Reference"))
  (bind _team (message `/Game/Blueprint/PlayerControllers/Interface_TeamPlayerController.GetTeam` Controller))
  (bind (_spawntransform _spawnactor _isfound) (`self.SpawnToTeam` _team))
  (if _isfound
    (bind _aspc_base (cast `/Game/Blueprint/PlayerControllers/PC_Base` Controller))
    (`/Game/Blueprint/Teams/BP_TankPlayerStart.LinkCurrentPCRef` _spawnactor _aspc_base)
    (bind _returnvalue (`|SpawnActorFromClass` "/Game/Blueprint/TankPawns/BP_PlayerTankBase.BP_PlayerTankBase_C" _spawntransform "Undefined" "OverrideRootScale" null null))
    (`Controller.Possess` _aspc_base _returnvalue)
    (else
      (`KismetSystemLibrary.PrintString` "can't find spawner"))))

(fn `SpawnToTeam`
  (params (TeamToSpawn :type "/Game/Blueprint/Teams/EnumTeams Enum" :default "NewEnumerator0") (PC :type "/Game/Blueprint/PlayerControllers/PC_Base Object Reference"))
  (returns (spawnTransform :type "Transform Structure (by ref)") (SpawnActor :type "/Game/Blueprint/Teams/BP_TankPlayerStart Object Reference") (isFound :type Boolean))
  (locals (LocalPC :type "/Game/Blueprint/PlayerControllers/PC_Base Object Reference"))
  (set `local.LocalPC` PC)
  (switch `/Game/Blueprint/Teams/EnumTeams` TeamToSpawn
    (:`NewEnumerator0`
      (bind (_location _playerstartref) (`self.GetSpawnerLocation` (`self.No Team Player Start Array`) (`local.LocalPC`))
        (:`Found `
          (return _location _playerstartref true))
        (:`NotFound`
          (return (struct) null false))))
    (:`NewEnumerator1`
      (bind (_location_2 _playerstartref_2) (`self.GetSpawnerLocation` (`self.Red Team Player Start Array`) (`local.LocalPC`))
        (:`Found `
          (return _location_2 _playerstartref_2 true))
        (:`NotFound`
          (return (struct) null false))))
    (:`NewEnumerator2`
      (bind (_location_3 _playerstartref_3) (`self.GetSpawnerLocation` (`self.Blue Team Player Start Array`) (`local.LocalPC`))
        (:`Found `
          (return _location_3 _playerstartref_3 true))
        (:`NotFound`
          (return (struct) null false))))))

(fn `UserConstructionScript`
  (`parent.UserConstructionScript`))