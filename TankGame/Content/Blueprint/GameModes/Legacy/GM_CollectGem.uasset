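; Game mode for a gem collection mode that triggers a win state once every gem in the level is collected.
; On BeginPlay it creates the in-game UI and binds each BP_Gem's collect event.
; Each pickup increments the count, checks for completion and sets the UI's gem count from that check.
; New players alternate between two teams via FlipFlop and are restarted until they control a valid pawn.
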(event `self.ReceiveBeginPlay`
  (`parent.ReceiveBeginPlay`)
  (`|ExecutionSequence`
    (:`then_0`
      (bind _returnvalue (`|CreateWidget` "/Game/Blueprint/HUD/UI_InGame_GemCollect.UI_InGame_GemCollect_C" (`GameplayStatics.GetPlayerController` 0)))
      (bind _output_get (set `self.In Game UI` _returnvalue))
      (`UserWidget.AddToViewport` _output_get 0))
    (:`then_1`
      ;[0.1955 0.3473 1 1 30] GAME MODE
      ;;[1 1 1] Gem Init
      (bind _outactors (`GameplayStatics.GetAllActorsOfClass` "/Game/Blueprint/Collectables/BP_Gem.BP_Gem_C"))
      (bind _output_get_2 (set `self.GemArray` _outactors))
      ;;[1 1 1] Gem Event Binding
      (for _array_element _output_get_2
        (add `/Game/Blueprint/Collectables/BP_Gem.CollectGemEvent` _array_element (delegate `OnCollectGem`))))
    (:`then_2`
      ;[1 1 1] Update UI on Start
      (`self.Update Gem UI`))))

(event `OnCollectGem`
  (params (`Gem Ref` :type "/Game/Blueprint/Collectables/BP_Gem Object Reference"))
  ;[0.1955 0.3473 1 1 30] GAME MODE
  ;;[1 1 1] Gem Event Logic
  (`|ExecutionSequence`
    (:`then_0`
      (`/Engine/EditorBlueprintResources/StandardMacros.IncrementInt` (`self.GemCollected`)
        (:`  `
          (`self.CheckAllGemCollected?`
            (:`true`
              (`self.Win State` null))))))
    (:`then_1`
      (`self.Update Gem UI`))))

(event `self.HandleStartingNewPlayer`
  (params (NewPlayer :type "PlayerController Object Reference"))
  (bind _aspc_gem_collect (cast `/Game/Blueprint/PlayerControllers/legacy/PC_GemCollect` NewPlayer))
  (`/Engine/EditorBlueprintResources/StandardMacros.FlipFlop`
    (:`A`
      (set `/Game/Blueprint/PlayerControllers/legacy/PC_GemCollect.Teams` "NewEnumerator1" _aspc_gem_collect))
    (:`B`
      (set `/Game/Blueprint/PlayerControllers/legacy/PC_GemCollect.Teams` "NewEnumerator2" _aspc_gem_collect)))
  (while (not (`KismetSystemLibrary.IsValid` (`Controller.K2_GetPawn` _aspc_gem_collect)))
    (`self.RestartPlayer` _aspc_gem_collect)))

(fn `UserConstructionScript`)