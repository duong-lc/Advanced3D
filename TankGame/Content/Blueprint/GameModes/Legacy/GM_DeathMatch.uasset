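; Legacy deathmatch game mode that spawns players at random BP_TankPlayerStart points, all reset to one team value, retrying restart until each has a pawn.
; It tracks controllers on login and logout, printing the last remaining player's pawn as winner.
; A one-second looping countdown prints a loss at zero.
; Gem-collect leftovers remain: timer and gem UI updates are stubs, and the created widget never reaches the viewport.
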(event `self.ReceiveBeginPlay`
  (for _ (range 0)
    (`GameplayStatics.CreatePlayer` -1))
  (`|ExecutionSequence`
    (:`then_0`
      (`|CreateWidget` "/Game/Blueprint/HUD/UI_InGame_GemCollect.UI_InGame_GemCollect_C" (`GameplayStatics.GetPlayerController` 0)))
    (:`then_1`
      ;[1 1 1] Update UI on Start
      (`self.Update Timer UI`))
    (:`then_3`
      (`KismetSystemLibrary.K2_SetTimerDelegate` (delegate `TimerCountDown`) 1.0 true))))

(event `Win State`
  (params (Winner :type "Pawn Object Reference"))
  (`KismetSystemLibrary.PrintString` (`KismetSystemLibrary.GetDisplayName` Winner)))

(event `TimerCountDown`
  (`/Engine/EditorBlueprintResources/StandardMacros.DecrementInt` (`self.Timer`)
    (:`  `
      (`self.Update Timer UI`)
      (`self.CheckTimerRanOut?`
        (:`true`
          (`self.Lose State`))))))

(event `Lose State`
  (`KismetSystemLibrary.PrintString` "You Lost"))

(event `self.HandleStartingNewPlayer`
  (params (NewPlayer :type "PlayerController Object Reference"))
  (bind _aspc_death_match (cast `/Game/Blueprint/PlayerControllers/legacy/PC_DeathMatch` NewPlayer))
  (while (not (`KismetSystemLibrary.IsValid` (`Controller.K2_GetPawn` _aspc_death_match)))
    (`self.RestartPlayer` _aspc_death_match)))

(event `self.K2_PostLogin`
  (params (NewPlayer :type "PlayerController Object Reference"))
  (`KismetArrayLibrary.Array_AddUnique` (`self.Players`) NewPlayer))

(event `self.K2_OnLogout`
  (params (ExitingController :type "Controller Object Reference"))
  (`KismetArrayLibrary.Array_RemoveItem` (`self.Players`) ExitingController)
  (if (== (`KismetArrayLibrary.Array_Length` (`self.Players`)) 1)
    (`self.Win State` (`Controller.K2_GetPawn` (`|GetArrayItem` (`self.Players`))))))

(fn `FindPlayerStart`
  (params (Player :type "Controller Object Reference") (IncomingName :type String))
  (returns (ReturnValue :type "Actor Object Reference"))
  (bind _outactors (`GameplayStatics.GetAllActorsOfClass` "/Game/Blueprint/Teams/BP_TankPlayerStart.BP_TankPlayerStart_C"))
  (for _array_element _outactors
    (set `/Game/Blueprint/Teams/BP_TankPlayerStart.Team` "NewEnumerator0" _array_element)
    (`KismetArrayLibrary.Array_AddUnique` (`self.No Team Player Start Array`) _array_element))
  (return (`KismetArrayLibrary.Array_Random` (`self.No Team Player Start Array`))))

(fn `UserConstructionScript`)