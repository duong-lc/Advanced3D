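; Game mode for a timed gem-collection challenge: collecting every gem wins, the countdown reaching zero loses.
; On BeginPlay it creates the HUD widget, binds to each BP_Gem's collect event and starts a looping one-second timer.
; Gem pickups and timer ticks update the widget's variables and run the win or lose checks.
; Both outcomes only print a message, and the timer is never stopped.
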(event `self.ReceiveBeginPlay`
  (`|ExecutionSequence`
    (:`then_0`
      (bind _returnvalue (`|CreateWidget` "/Game/Blueprint/HUD/UI_InGame_GemCollect.UI_InGame_GemCollect_C" (`GameplayStatics.GetPlayerController` 0)))
      (bind _output_get (set `self.In Game UI` _returnvalue))
      (`UserWidget.AddToViewport` _output_get 0))
    (:`then_1`
      ;[0.1955 0.3473 1 1 30] GAME MODE
      ;;[1 1 1] Gem Init
      (bind _outactors (`GameplayStatics.GetAllActorsOfClass` "/Game/Blueprint/Collectables/BP_Gem.BP_Gem_C"))
      (bind _output_get_2 (set `self.GemArray` _outactors))
      ;;[1 1 1] Gem Event Binding
      (for _array_element _output_get_2
        (add `/Game/Blueprint/Collectables/BP_Gem.CollectGemEvent` _array_element (delegate `OnCollectGem`))))
    (:`then_2`
      ;[1 1 1] Update UI on Start
      (`self.Update Gem UI`)
      (`self.Update Timer UI`))
    (:`then_3`
      (`KismetSystemLibrary.K2_SetTimerDelegate` (delegate `TimerCountDown`) 1.0 true))))

(event `Win State`
  (`KismetSystemLibrary.PrintString` "You Win"))

(event `Lose State`
  (`KismetSystemLibrary.PrintString` "You Lost"))

(event `OnCollectGem`
  (params (`Gem Ref` :type "/Game/Blueprint/Collectables/BP_Gem Object Reference"))
  ;[0.1955 0.3473 1 1 30] GAME MODE
  ;;[1 1 1] Gem Event Logic
  (`|ExecutionSequence`
    (:`then_0`
      (`/Engine/EditorBlueprintResources/StandardMacros.IncrementInt` (`self.GemCollected`)
        (:`  `
          (`self.CheckAllGemCollected?`
            (:`true`
              (`self.Win State`))))))
    (:`then_1`
      (`self.Update Gem UI`))))

(event `TimerCountDown`
  (`/Engine/EditorBlueprintResources/StandardMacros.DecrementInt` (`self.Timer`)
    (:`  `
      (`self.Update Timer UI`)
      (`self.CheckTimerRanOut?`
        (:`true`
          (`self.Lose State`))))))

(fn `UserConstructionScript`)