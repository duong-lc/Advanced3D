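; GM_TurfWar is the game mode for a timed Turf War match decided by which team owns the most tiles.
; It caches all BP_Tile actors in its construction script and restarts each new PC_TurfWar player until it has a pawn.
; LoseState tallies red and blue tile ownership and prints the counts and winner or tie, while WinState just prints the winner's name.
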(event `self.ReceiveBeginPlay`
  (set `self.isGameTimeOrientated` true)
  (`parent.ReceiveBeginPlay`))

(event `Win State`
  (params (Winner :type "Pawn Object Reference"))
  (`KismetSystemLibrary.PrintString` (`KismetSystemLibrary.GetDisplayName` Winner)))

(event `Lose State`
  (`self.LoseState`))

(event `self.HandleStartingNewPlayer`
  (params (NewPlayer :type "PlayerController Object Reference"))
  (bind _aspc_turf_war (cast `/Game/Blueprint/PlayerControllers/PC_TurfWar` NewPlayer))
  (while (not (`KismetSystemLibrary.IsValid` (`Controller.K2_GetPawn` _aspc_turf_war)))
    (`self.RestartPlayer` _aspc_turf_war)))

(fn `LoseState`
  (locals (RedTiles :type Integer) (BlueTiles :type Integer))
  (`KismetSystemLibrary.PrintString` "You Lost" true true (struct :`R` 1.0 :`G` 0.009923 :`B` 0.03977 :`A` 1.0))
  (for _array_element (`self.AllTiles`)
    (switch `/Game/Blueprint/Teams/EnumTeams` (`/Game/Blueprint/TurfWar/BP_Tile.TeamOwning` _array_element)
      (:`NewEnumerator1`
        (`/Engine/EditorBlueprintResources/StandardMacros.IncrementInt` (`local.RedTiles`)))
      (:`NewEnumerator2`
        (`/Engine/EditorBlueprintResources/StandardMacros.IncrementInt` (`local.BlueTiles`)))))
  (`KismetSystemLibrary.PrintString` (`KismetStringLibrary.Concat_StrStr` "red: " (`KismetStringLibrary.Conv_IntToString` (`local.RedTiles`))))
  (`KismetSystemLibrary.PrintString` (`KismetStringLibrary.Concat_StrStr` "blue: " (`KismetStringLibrary.Conv_IntToString` (`local.BlueTiles`))))
  (if (> (`local.RedTiles`) (`local.BlueTiles`))
    (`KismetSystemLibrary.PrintString` "RED WINS")
    (elif (== (`local.RedTiles`) (`local.BlueTiles`))
      (`KismetSystemLibrary.PrintString` "TIES")
      (else
        (`KismetSystemLibrary.PrintString` "BLUE WINS")))))

(fn `UserConstructionScript`
  (bind _outactors (`GameplayStatics.GetAllActorsOfClass` "/Game/Blueprint/TurfWar/BP_Tile.BP_Tile_C"))
  (set `self.AllTiles` _outactors))