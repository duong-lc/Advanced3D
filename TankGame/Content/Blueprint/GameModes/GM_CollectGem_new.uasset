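; Game mode for a timed Gem Collect match with local players and AI, all assigned to no team.
; Local player count comes from the options string, with AI filling toward the match maximum.
; BeginPlay caches gems, spawns player tanks with per-player HUD and team-tinted cursor, then moves AI pawns to spawn points.
; A ready-up overlay pauses play; LoseState pauses and shows the end screen, while WinState only prints the winner.
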(event `self.ReceiveBeginPlay`
  (set `self.Timer` 30)
  (set `self.isGameTimeOrientated` true)
  (`parent.ReceiveBeginPlay`)
  (`self.SetupGemCollectGMRef`)
  (`self.SetUpPlayerSpawnRefs`)
  (`|ExecutionSequence`
    (:`then_0`
      (for _array_element (`self.All Players`)
        (`KismetSystemLibrary.PrintString` "Spawning Player OBJ")
        (`self.Spawn Player` _array_element)))
    (:`then_1`
      (`self.Spawn All AI`))
    (:`then_2`
      (bind _returnvalue (`|CreateWidget` (`self.UIEnd Screen Class`)))
      (set `self.UIEndScreenRef` _returnvalue))
    (:`then_3`
      (message `/Game/Blueprint/GameModes/GM_Multiplayer_Interface.OnReadyUpOn` self))))

(event `Win State`
  (params (Winner :type "Pawn Object Reference"))
  (`KismetSystemLibrary.PrintString` (`KismetSystemLibrary.GetDisplayName` Winner)))

(event `Lose State`
  (`self.LoseState`))

(event `self.ReceiveTick`
  (params (DeltaSeconds :type "Float (single-precision)")))

(event `/Game/Blueprint/GameModes/GM_Multiplayer_Interface.OnReadyUpOff`
  (`Widget.RemoveFromParent` (`self.ReadyUpOverlayRef`))
  (`GameplayStatics.SetGamePaused` false))

(event `/Game/Blueprint/GameModes/GM_Multiplayer_Interface.OnReadyUpOn`
  (bind _readyupoverlayref (`self.ReadyUpOverlayRef`))
  (`UserWidget.AddToViewport` _readyupoverlayref 0)
  (`/Game/Blueprint/UI_AllGMReadyUpOverlay.OnDisplayReadyUp` _readyupoverlayref (+ (`self.localPlayersCount`) 2))
  (`GameplayStatics.SetGamePaused` true)
  (`/Game/Blueprint/UI_AllGMReadyUpOverlay.Player Ready Up On` (`self.ReadyUpOverlayRef`))
  (`/Game/Blueprint/UI_AllGMReadyUpOverlay.Player Ready Up Off` (`self.ReadyUpOverlayRef`)))

(event `/Game/Blueprint/GameModes/GM_Multiplayer_Interface.OnReadyUpInput`
  (params (ReadyState :type Boolean))
  (if ReadyState
    (`/Game/Blueprint/UI_AllGMReadyUpOverlay.Player Ready Up On` (`self.ReadyUpOverlayRef`))
    (else
      (`/Game/Blueprint/UI_AllGMReadyUpOverlay.Player Ready Up Off` (`self.ReadyUpOverlayRef`)))))

(fn `AddTotalPlayers`
  (locals (playerCountTemp :type Integer :default 0) (`is A` :type Boolean :default false))
  (if (> (`self.maxPlayerInGame`) 0)
    (bind _output_get (set `self.localPlayersCount` (- (`KismetStringLibrary.Conv_StringToInt` (`GameplayStatics.ParseOption` (`self.OptionsString`) "players")) 2)))
    (set `self.AIPlayerCount` (- (`self.maxPlayerInGame`) (`self.localPlayersCount`)))
    (for _ (range (+ _output_get 1))
      (bind _aspc_base (`self.AddLocalPlayer`))
      (`/Game/Blueprint/PlayerControllers/PC_Base.SetTeam` _aspc_base "NewEnumerator0")
      (message `/Game/Blueprint/PlayerControllers/Interface_TeamPlayerController.SetTeam` _aspc_base "NewEnumerator0"))))

(fn `Initialize AI Pawn`
  (params (`Ai Controller` :type "/Game/Blueprint/EnemyMob/GemCollect/AIC_GemCollect Object Reference") (TeamToSpawn :type "/Game/Blueprint/Teams/EnumTeams Enum" :default "NewEnumerator0"))
  (returns (`Spawn Success?` :type Boolean))
  (bind (_spawntransform _spawnactor _isfound) (`self.Get AI Spawn Point` TeamToSpawn `Ai Controller`))
  (message `/Game/Blueprint/PlayerControllers/Interface_TeamPlayerController.SetTeam` `Ai Controller` TeamToSpawn)
  (if _isfound
    (`self.K2_SetActorTransform` (`Controller.K2_GetPawn` `Ai Controller`) _spawntransform false true)
    (bind _aic_ref (`/Game/Blueprint/Teams/BP_TankPlayerStart.Link Current AIC Ref` _spawnactor `Ai Controller`))
    (message `/Game/Blueprint/PlayerControllers/Interface_TeamPlayerController.SetPlayerStart` _aic_ref _spawnactor))
  (return _isfound))

(fn `LoseState`
  (bind _uiendscreenref (`self.UIEndScreenRef`))
  (`KismetSystemLibrary.PrintString` "Collect Gem game mode ended" true true (struct :`R` 1.0 :`G` 0.009923 :`B` 0.03977 :`A` 1.0))
  (`/Game/Blueprint/Collectables/UI_EndGame_GemCollect.UpdateEndGameStats` _uiendscreenref)
  (bind _asplayer_controller (cast `PlayerController` (`|GetArrayItem` (`self.All Players`))))
  (set `PlayerController.bShowMouseCursor` true _asplayer_controller)
  (`GameplayStatics.SetGamePaused` true)
  (`UserWidget.AddToViewport` _uiendscreenref 0))

(fn `SetupGemCollectGMRef`
  (`|ExecutionSequence`
    (:`then_0`
      (bind _outactors (`GameplayStatics.GetAllActorsOfClass` "/Game/Blueprint/Collectables/BP_Gem.BP_Gem_C"))
      (set `self.AllGems` _outactors))))

(fn `SetUpUIMouseCursor`
  (params (Controller :type "Controller Object Reference"))
  (bind _ui_instance (`parent.SetUpUIMouseCursor` Controller))
  (bind _team (message `/Game/Blueprint/PlayerControllers/Interface_TeamPlayerController.GetTeam` (`/Game/Blueprint/PlayerControllers/UI_MouseCursor.PC inst` _ui_instance)))
  (switch `/Game/Blueprint/Teams/EnumTeams` _team
    (:`NewEnumerator0`
      (bind _mousecursor (`/Game/Blueprint/PlayerControllers/UI_MouseCursor.MouseCursor` _ui_instance))
      (`Image.SetColorAndOpacity` _mousecursor (struct :`R` 0.987301 :`G` 1.0 :`B` 0.934119 :`A` 1.0)))
    (:`NewEnumerator1`
      (`Image.SetColorAndOpacity` _mousecursor (struct :`R` 1.0 :`B` 0.13424 :`A` 1.0)))
    (:`NewEnumerator2`
      (`Image.SetColorAndOpacity` _mousecursor (struct :`G` 0.77537 :`B` 1.0 :`A` 1.0)))))

(fn `Spawn All AI`
  (for _ (range 1 (+ (- (`self.AIPlayerCount`) 2) 1))
    (bind _returnvalue (`|SpawnActorFromClass` "/Game/Blueprint/EnemyMob/GemCollect/P_AI_GemCollect.P_AI_GemCollect_C" (`KismetMathLibrary.MakeTransform` (0.0 0.0 110.0)) "AlwaysSpawn" "OverrideRootScale" null null))
    (`KismetSystemLibrary.PrintString` (`KismetSystemLibrary.GetDisplayName` _returnvalue))
    (bind _ai_controller (`/Game/Blueprint/EnemyMob/GemCollect/P_AI_GemCollect.Get AI Controller` _returnvalue))
    (`KismetArrayLibrary.Array_AddUnique` (`self.All AI Controllers`) _ai_controller))
  (for _array_element (`self.All AI Controllers`)
    (bind _asaic_gem_collect (cast `/Game/Blueprint/EnemyMob/GemCollect/AIC_GemCollect` _array_element))
    (`self.Initialize AI Pawn` _asaic_gem_collect)))

(fn `Spawn Player`
  (params (Controller :type "Controller Object Reference"))
  (locals (UI_Inst :type "/Game/Blueprint/Collectables/UI_InGame_CollectGem Object Reference"))
  (bind _aspc_gem_collect_new (cast `/Game/Blueprint/PlayerControllers/PC_GemCollect_new` Controller))
  (bind _team (message `/Game/Blueprint/PlayerControllers/Interface_TeamPlayerController.SetTeam` _aspc_gem_collect_new "NewEnumerator0"))
  (bind (_spawntransform _spawnactor _isfound) (`self.Get Player Spawn Point` _team _aspc_gem_collect_new))
  (if _isfound
    (bind _pcref (`/Game/Blueprint/Teams/BP_TankPlayerStart.Link Current PC Ref` _spawnactor _aspc_gem_collect_new))
    (set `/Game/Blueprint/PlayerControllers/PC_Base.CurrentSpawner` _spawnactor _pcref)
    (bind _returnvalue (`|SpawnActorFromClass` "/Game/Blueprint/TankPawns/GemCollectPawns/P_TankCollectGem.P_TankCollectGem_C" _spawntransform "Undefined" "OverrideRootScale" null null))
    (bind _returnvalue_2 (`|CreateWidget` "/Game/Blueprint/Collectables/UI_InGame_CollectGem.UI_InGame_CollectGem_C" _aspc_gem_collect_new))
    (bind _output_get (set `local.UI_Inst` _returnvalue_2))
    (set `/Game/Blueprint/Collectables/UI_InGame_CollectGem.PC_inst` _aspc_gem_collect_new _output_get)
    (`UserWidget.AddToPlayerScreen` _output_get 0)
    (`self.SetUpUIMouseCursor` _aspc_gem_collect_new)
    (set `/Game/Blueprint/PlayerControllers/PC_GemCollect_new.UI_Inst` _output_get _aspc_gem_collect_new)
    (`KismetSystemLibrary.PrintString` "POSSESS gem pawn")
    (`Controller.Possess` _aspc_gem_collect_new _returnvalue)
    (else
      (`KismetSystemLibrary.PrintString` "can't find spawner"))))

(fn `UserConstructionScript`)