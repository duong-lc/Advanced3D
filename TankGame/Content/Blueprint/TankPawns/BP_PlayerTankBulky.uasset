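; BP_PlayerTankBulky is the bulky player tank variant, configured with its own health, material, speed and enlarged scale.
; All setup runs in the Construction Script, which calls ResetToNone and then applies each stat and look through setter functions.
; The event graph holds only disabled placeholder events, so the Blueprint adds no runtime logic of its own.
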(fn `UserConstructionScript`
  (`self.Reset to None`)
  (`self.SetMaxHealth` 200.0)
  (`self.SetMaterial` "/Game/Assets/EnemyMesh/En_Mat01_2_Inst1.En_Mat01_2_Inst1")
  (`self.SetSpeed` 0.2)
  (`self.SetScale` (1.5 1.5 1.5)))