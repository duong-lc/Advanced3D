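; BP_PlayerTankNimble is a player tank pawn variant that, as its name suggests, trades toughness for agility.
; The construction script calls ResetToNone, then configures max health, material, speed and a half-size uniform scale through setter functions.
; The event graph holds only disabled placeholder events, so this Blueprint adds no runtime logic of its own.
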(fn `UserConstructionScript`
  (`self.Reset to None`)
  (`self.SetMaxHealth` 50.0)
  (`self.SetMaterial` "/Game/Assets/EnemyMesh/En_Mat01_2_Inst.En_Mat01_2_Inst")
  (`self.SetSpeed` 0.8)
  (`self.SetScale` (0.5 0.5 0.5)))