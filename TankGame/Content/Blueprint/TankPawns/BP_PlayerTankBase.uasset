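; Base player tank pawn that holds health, speed and scale, and manages the weapons the player picks up and cycles through.
; InventoryComponent slots track ammo and cooldowns, while switching releases the current weapon to its slot and retrieves the next.
; Pickups are added to the inventory, with duplicates destroyed after equipping the stored copy.
; Equipped weapons snap to the turretPivot socket and notify the controller; death only prints, and material setup is disconnected.
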(event `self.ReceiveTick`
  (params (DeltaSeconds :type "Float (single-precision)")))

(event `/Game/Blueprint/PlayerInterface.InitiateCurrentCoolDown`
  (params (`Firing Weapon` :type "/Game/Blueprint/Enums/EnumWeaponType Enum" :default "NewEnumerator4"))
  (if (`|EnumEquality` `Firing Weapon` (`self.CurrentWeaponType`))
    (`/Game/Blueprint/InventorySystem/BP_InventoryComponent.InitiateSlotCooldown` (`self.InventoryComponent`) (`self.CurrentWeaponType`))
    (else
      (`KismetSystemLibrary.PrintString` "Weapon firing not the same as current weapon in pawn" true true (struct :`R` 1.0 :`G` 0.083106 :`A` 1.0)))))

(event `/Game/Blueprint/PlayerInterface.ChangeToWeapon`
  (params (newWeaponType :type "/Game/Blueprint/Enums/EnumWeaponType Enum" :default "NewEnumerator4"))
  (`KismetSystemLibrary.PrintString` (`KismetStringLibrary.Concat_StrStr` (`|GetEnumeratorNameAsString` newWeaponType) "CHANGE TO"))
  ;[0.7706 1 0.99] 1. Get Slot of Weapon To Switch
  (bind (_inventory_slot _is_valid) (`/Game/Blueprint/InventorySystem/BP_InventoryComponent.Get Slot` (`self.InventoryComponent`) newWeaponType))
  (if _is_valid
    ;[0.4671 1 0.9602] 2. Get Slot of Current weapon and release it back to slot
    (bind (_inventory_slot_2 _is_valid_2) (`/Game/Blueprint/InventorySystem/BP_InventoryComponent.Get Slot` (`self.InventoryComponent`) (`self.CurrentWeaponType`)))
    (if _is_valid_2
      (`/Game/Blueprint/InventorySystem/BP_InventorySlot.ReleaseWeaponBackToSlot` _inventory_slot_2 (`self.CurrentWeaponRef`))
      (else
        (`KismetSystemLibrary.PrintString` "Slot Doesn't exist 2nd")))
    ;[0 1 0.9555] 3. Get Weapon from Slot
    (bind _pickupref (`/Game/Blueprint/InventorySystem/BP_InventorySlot.GetWeaponFromSlot` _inventory_slot))
    (`self.UpdateCurrentWeapon` _pickupref)
    (else
      (`KismetSystemLibrary.PrintString` "Slot Doesn't exist 1st"))))

(event `/Game/Blueprint/PlayerInterface.ChangeToNextWeapon`
  (bind (_slot _next_weapon_enum) (`/Game/Blueprint/InventorySystem/BP_InventoryComponent.Get Next Item` (`self.InventoryComponent`) (`self.CurrentWeaponType`)))
  (if true
    (`/Game/Blueprint/PlayerInterface.ChangeToWeapon` _next_weapon_enum)
    (else
      (`KismetSystemLibrary.PrintString` "Can't Cycle Next" true true (struct :`R` 1.0 :`G` 0.028928 :`A` 1.0)))))

(event `/Game/Blueprint/PlayerInterface.ChangeToPrevWeapon`
  (bind (_slot _previous_weapon_enum _shouldcycle) (`/Game/Blueprint/InventorySystem/BP_InventoryComponent.GetPreviousItem` (`self.InventoryComponent`) (`self.CurrentWeaponType`)))
  (if _shouldcycle
    (`/Game/Blueprint/PlayerInterface.ChangeToWeapon` _previous_weapon_enum)
    (else
      (`KismetSystemLibrary.PrintString` "Can't Cycle Prev" true true (struct :`R` 1.0 :`G` 0.028928 :`A` 1.0)))))

(event `/Game/Blueprint/PlayerInterface.OnWeaponPickUp`
  (params (`Weapon To PickUp` :type "/Game/Blueprint/WeaponPickUp/BP_PickUpBase Object Reference"))
  (`self.On Weapon Pick Up` `Weapon To PickUp`))

(fn `GetCurrentCoolDown`
  (returns (canShoot :type Boolean) (coolDown :type "Float (double-precision)"))
  (bind (_canshoot _cooldownpercent) (`/Game/Blueprint/InventorySystem/BP_InventoryComponent.CheckCanShoot` (`self.InventoryComponent`) (`self.CurrentWeaponType`)))
  (return _canshoot _cooldownpercent))

(fn `GetCurrentWeapon`
  (params (WeaponType :type "/Game/Blueprint/Enums/EnumWeaponType Enum" :default "NewEnumerator4"))
  (returns (`Weapon Ref` :type "/Game/Blueprint/WeaponPickUp/BP_PickUpBase Object Reference") (IsFound :type Boolean))
  (bind (_value _isfound) (`/Game/Blueprint/InventorySystem/BP_InventoryComponent.GetSlotByType` (`self.InventoryComponent`) WeaponType))
  (if (`|EnumInequality` WeaponType "NewEnumerator4")
    (if _isfound
      (return (`/Game/Blueprint/InventorySystem/BP_InventorySlot.PickUpRef` _value) _isfound)
      (else
        _)))
  (return null false))

(fn `GetHealth`
  (returns (Health :type "Float (double-precision)"))
  (return (`self.Health`)))

(fn `GetWeaponStats`
  (returns (WeaponType :type "/Game/Blueprint/Enums/EnumWeaponType Enum") (Ammo :type Integer))
  (bind (_inventory_slot _is_valid) (`/Game/Blueprint/InventorySystem/BP_InventoryComponent.Get Slot` (`self.InventoryComponent`) (`self.CurrentWeaponType`)))
  (if _is_valid
    (return (`self.CurrentWeaponType`) (`/Game/Blueprint/InventorySystem/BP_InventorySlot.GetAmmo` _inventory_slot))
    (else
      (return (`self.CurrentWeaponType`) 0))))

(fn `IsOverlapping`
  (returns (isOverlapping :type Boolean))
  (return (> (`KismetArrayLibrary.Array_Length` (`PrimitiveComponent.GetOverlappingActors` (`self.CapsuleComponent`) "BP_PlayerTankBase_C")) 1)))

(fn `On Weapon Pick Up`
  (params (Weapon :type "/Game/Blueprint/WeaponPickUp/BP_PickUpBase Object Reference"))
  (locals (pickedUpWeapon :type "/Game/Blueprint/WeaponPickUp/BP_PickUpBase Object Reference") (CurrentInventorySlot :type "/Game/Blueprint/InventorySystem/BP_InventorySlot Object Reference") (CurrentInventoryFound :type Boolean :default false))
  (set `local.pickedUpWeapon` Weapon)
  ;[1 0.3434 0.3633] Get Current Inven Slot. True -> alr exist. False -> not picked up -> Add new
  (bind (_inventory_slot _is_valid) (`/Game/Blueprint/InventorySystem/BP_InventoryComponent.Get Slot` (`self.InventoryComponent`) (`self.CurrentWeaponType`)))
  (set `local.CurrentInventorySlot` _inventory_slot)
  (bind _output_get (set `local.CurrentInventoryFound` _is_valid))
  (if _output_get
    ;[1 0.3434 0.3633] Check null ref current weapon global
    (`/Engine/EditorBlueprintResources/StandardMacros.IsValid` (`local.pickedUpWeapon`)
      (:`Is Valid`
        (`/Engine/EditorBlueprintResources/StandardMacros.IsValid` (`self.CurrentWeaponRef`)
          (:`Is Valid`
            ;[1 0.3434 0.3633] Check if Ref in inventory == picked up ref
            (if (== (`self.CurrentWeaponRef`) (`/Game/Blueprint/InventorySystem/BP_InventorySlot.PickUpRef` (`local.CurrentInventorySlot`)))
              ;[1 0.3434 0.3633] Move Current Global to attach to inventory
              (`/Game/Blueprint/InventorySystem/BP_InventorySlot.ReleaseWeaponBackToSlot` (`local.CurrentInventorySlot`) (`self.CurrentWeaponRef`))
              ;[0.1357 0.7785 1] Check Picked Up Weapon alr in inventory or not
              (bind (_inventory_slot_2 _is_valid_2) (`/Game/Blueprint/InventorySystem/BP_InventoryComponent.Get Slot` (`self.InventoryComponent`) (`/Game/Blueprint/WeaponPickUp/BP_PickUpBase.WeaponType` (`local.pickedUpWeapon`))))
              ;[0.1357 0.7785 1] if it's alr exist -> Unparent & make visible from the slot
              (if _is_valid_2
                (bind _pickupref (`/Game/Blueprint/InventorySystem/BP_InventorySlot.GetWeaponFromSlot` _inventory_slot_2))
                (`/Game/Blueprint/InventorySystem/BP_InventoryComponent.AddItem` (`self.InventoryComponent`) (`local.pickedUpWeapon`))
                (`self.UpdateCurrentWeapon` _pickupref)
                (`KismetSystemLibrary.PrintString` "attached")
                (`self.K2_DestroyActor` (`local.pickedUpWeapon`))
                (else
                  ;[1 1 1] Add to Inventory
                  (`/Game/Blueprint/InventorySystem/BP_InventoryComponent.AddItem` (`self.InventoryComponent`) (`local.pickedUpWeapon`) :!label _label)
                  (`self.UpdateCurrentWeapon` (`local.pickedUpWeapon`))
                  (`KismetSystemLibrary.PrintString` "attached")))
              (else
                (`KismetSystemLibrary.PrintString` "NOT SAME WEAPON REF"))))
          (:`Is Not Valid`
            (`KismetSystemLibrary.PrintString` "REF IS NULL"))))
      (:`Is Not Valid`
        (`KismetSystemLibrary.PrintString` "Picked up ref is null")))
    (else
      (goto _label))))

(fn `Reset to None`)

(fn `SetMaterial`
  (params (Material :type "MaterialInterface Object Reference") (isInvis :type Boolean)))

(fn `SetMaxHealth`
  (params (maxHealth :type "Float (double-precision)"))
  (bind _output_get (set `self.maxHealth` maxHealth))
  (set `self.Health` _output_get))

(fn `SetScale`
  (params (NewScale :type "Vector Structure"))
  (`SceneComponent.SetWorldScale3D` (`self.Body`) NewScale))

(fn `SetSpeed`
  (params (speed :type "Float (double-precision)"))
  (set `self.speed` speed))

(fn `TakeDamage`
  (params (damageTaken :type "Float (double-precision)"))
  (returns (`Health Returned` :type "Float (double-precision)"))
  (bind _output_get (set `self.Health` (- (`self.Health`) damageTaken)))
  (if (<= _output_get 0.0)
    (`KismetSystemLibrary.PrintString` "playerDead")
    (bind _output_get_2 (set `self.Health` 0.0))
    (return _output_get_2)
    (else
      (`KismetSystemLibrary.PrintString` "player not dead")
      (return (`self.Health`)))))

(fn `UserConstructionScript`
  (`self.Reset to None`)
  (`self.SetMaxHealth` 100.0)
  (`self.SetMaterial` "/Game/Assets/EnemyMesh/En_Mat01_2.En_Mat01_2")
  (`self.SetSpeed` 0.5)
  (`self.SetScale` (1.0 1.0 1.0)))