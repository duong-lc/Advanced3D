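; BP_PlayerTankInvisible is a player tank pawn variant that takes on an invisible look.
; Its construction script resets the tank to none, then sets max health, an alpha material flagged as invisible, speed and a uniform scale.
; The event graph holds only disabled parent-call stubs, so the Blueprint adds no runtime logic of its own.
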(fn `UserConstructionScript`
  (`self.Reset to None`)
  (`self.SetMaxHealth` 100.0)
  (`self.SetMaterial` "/Game/Assets/EnemyMesh/AlphaMat.AlphaMat" true)
  (`self.SetSpeed` 0.5)
  (`self.SetScale` (1.0 1.0 1.0)))