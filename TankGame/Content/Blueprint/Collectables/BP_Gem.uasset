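; BP_Gem is a collectable gem that awards a point to the pawn that touches it, existing only under the GM_CollectGem_new game mode.
; It destroys itself on BeginPlay in any other mode.
; When CanCollect is set, a sphere overlap sends AddPointToPawnMessage to the pawn, then hides the mesh and disables overlap events.
; A five-second delay restores both, so the gem respawns in place without being destroyed.
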(event `self.ReceiveBeginPlay`
  (cast `/Game/Blueprint/GameModes/GM_CollectGem_new` (`GameplayStatics.GetGameMode`)
    (:`CastFailed`
      (`self.K2_DestroyActor`))))

(event `self.Sphere.OnComponentBeginOverlap`
  (params (OverlappedComponent :type "PrimitiveComponent Object Reference") (OtherActor :type "Actor Object Reference") (OtherComp :type "PrimitiveComponent Object Reference") (OtherBodyIndex :type Integer) (bFromSweep :type Boolean) (SweepResult :type "HitResult Structure (by ref)"))
  (bind _aspawn (cast `Pawn` OtherActor))
  (if (`self.canCollect`)
    (message `/Game/Blueprint/Collectables/P_GemInteraction_Interface.AddPointToPawn` _aspawn 1)
    (set `PrimitiveComponent.bGenerateOverlapEvents` false (`self.Sphere`))
    (`SceneComponent.SetVisibility` (`self.StaticMesh`) false false)
    (`KismetSystemLibrary.Delay` 5.0)
    (set `PrimitiveComponent.bGenerateOverlapEvents` true (`self.Sphere`))
    (`SceneComponent.SetVisibility` (`self.StaticMesh`) true false)))

(fn `UserConstructionScript`)