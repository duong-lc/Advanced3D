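; Rocket projectile that flies between two given points and explodes on arrival or on overlapping a Pawn, skipping anything tagged "ignoreBullet".
; TraverseRocket attaches a trail emitter and drives position with a timeline lerp, without sweep.
; OnExplode disables overlaps, hides the rocket, spawns a hit effect and damages everything in EnemyArray, which is filled outside these graphs.
; Lifespan is set inside that damage loop, so only when the array has entries.
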(event `TraverseRocket`
  (params (start :type "Vector Structure") (end :type "Vector Structure"))
  (bind _returnvalue (`GameplayStatics.SpawnEmitterAttached` "/Game/Assets/Particles/ArtilleryTrailPAR.ArtilleryTrailPAR" (`self.Sphere`)))
  (set `self.trail` _returnvalue)
  (bind (_direction _alpha) (`Timeline|lerpAlpha` :!via `PlayFromStart`)
    (:`Update`
      (`self.K2_SetActorLocation` (`KismetMathLibrary.VLerp` start end _alpha)))
    (:`Finished`
      (`self.OnExplode`))))

(event `self.Sphere.OnComponentBeginOverlap`
  (params (OverlappedComponent :type "PrimitiveComponent Object Reference") (OtherActor :type "Actor Object Reference") (OtherComp :type "PrimitiveComponent Object Reference") (OtherBodyIndex :type Integer) (bFromSweep :type Boolean) (SweepResult :type "HitResult Structure (by ref)"))
  (if (not (or (`self.ActorHasTag` OtherActor "ignoreBullet") (`ActorComponent.ComponentHasTag` OtherComp "ignoreBullet")))
    (cast `Pawn` OtherActor)
    (`self.OnExplode`)))

(fn `OnExplode`
  (bind _ownercontroller (`self.OwnerController`))
  (set `PrimitiveComponent.bGenerateOverlapEvents` false (`self.DamageSphere`))
  (set `PrimitiveComponent.bGenerateOverlapEvents` false (`self.Sphere`))
  (`SceneComponent.SetVisibility` (`self.trail`) false false)
  (`SceneComponent.SetVisibility` (`self.StaticMesh`) false false)
  (`GameplayStatics.SpawnEmitterAtLocation` "/Game/Assets/Particles/RockBombHitPAR.RockBombHitPAR" (`self.K2_GetActorLocation`) (struct) (1.5 1.5 1.5))
  (for _array_element (`self.enemyArray`)
    (`KismetSystemLibrary.PrintString` (`KismetSystemLibrary.GetDisplayName` _ownercontroller))
    (`GameplayStatics.ApplyDamage` _array_element (`self.damage`) null _ownercontroller)
    (`self.SetLifeSpan` 2.0)))

(fn `UserConstructionScript`
  (`self.SetDamage` 100.0))