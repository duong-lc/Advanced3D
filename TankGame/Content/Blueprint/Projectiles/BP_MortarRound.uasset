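; Mortar round projectile that arcs from a start to an end point and explodes on arrival or on pawn contact.
; OnSpawn attaches a trail and runs two timelines: one lerps position, the other adds height, with rotation aimed along the path.
; An event track enables collision overlaps mid-flight.
; OnExplode hides the round, spawns a hit effect and damages EnemyArray actors; its TileArray loop is empty and SetLifeSpan is unconnected.
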(event `OnSpawn`
  (params (`start vect` :type "Vector Structure") (`end Vect` :type "Vector Structure"))
  (set `PrimitiveComponent.bGenerateOverlapEvents` false (`self.DamageSphere`))
  (set `PrimitiveComponent.bGenerateOverlapEvents` false (`self.Sphere`))
  (bind _returnvalue (`GameplayStatics.SpawnEmitterAttached` "/Game/Assets/Particles/ArtilleryTrailPAR.ArtilleryTrailPAR" (`self.Sphere`)))
  (set `self.trail` _returnvalue)
  (`|ExecutionSequence`
    (:`then_0`
      (bind (_direction _heightmod) (`Timeline|Timeline_0` :!via `PlayFromStart`)))
    (:`then_1`
      (bind (_direction_2 _alpha1) (`Timeline|Timeline_1` :!via `PlayFromStart`)
        (:`Update`
          (bind _returnvalue_2 (+ _heightmod (`KismetMathLibrary.VLerp` `start vect` `end Vect` _alpha1)))
          (`self.K2_SetActorRotation` (`KismetMathLibrary.FindLookAtRotation` (`self.K2_GetActorLocation`) _returnvalue_2))
          (`self.K2_SetActorLocation` _returnvalue_2))
        (:`Finished`
          (if (not (`self.isExplode`))
            (`self.OnExplode`)))
        (:`NewTrack_0`
          (set `PrimitiveComponent.bGenerateOverlapEvents` true (`self.DamageSphere`))
          (set `PrimitiveComponent.bGenerateOverlapEvents` true (`self.Sphere`)))))))

(event `self.Sphere.OnComponentBeginOverlap`
  (params (OverlappedComponent :type "PrimitiveComponent Object Reference") (OtherActor :type "Actor Object Reference") (OtherComp :type "PrimitiveComponent Object Reference") (OtherBodyIndex :type Integer) (bFromSweep :type Boolean) (SweepResult :type "HitResult Structure (by ref)"))
  (if (not (or (`self.ActorHasTag` OtherActor "ignoreBullet") (`ActorComponent.ComponentHasTag` OtherComp "ignoreBullet")))
    (cast `Pawn` OtherActor)
    (if (not (`self.isExplode`))
      (`self.OnExplode`))))

(fn `OnExplode`
  (locals (explodePos :type "Vector Structure" :default (0.0 0.0 0.0)))
  (set `self.isExplode` true)
  (set `local.explodePos` (`SceneComponent.K2_GetComponentLocation` (`self.Sphere`)))
  (set `PrimitiveComponent.bGenerateOverlapEvents` false (`self.DamageSphere`))
  (set `PrimitiveComponent.bGenerateOverlapEvents` false (`self.Sphere`))
  (`SceneComponent.SetVisibility` (`self.trail`) false false)
  (`SceneComponent.SetVisibility` (`self.StaticMesh`) false false)
  (`GameplayStatics.SpawnEmitterAtLocation` "/Game/Assets/Particles/RockBombHitPAR.RockBombHitPAR" (`local.explodePos`))
  (`|ExecutionSequence`
    (:`then_0`
      (for _array_element (`self.enemyArray`)
        (`GameplayStatics.ApplyDamage` _array_element (`self.damage`) null (`self.OwnerController`))))
    (:`then_1`
      (for _ (`self.TileArray`)
        _))))

(fn `UserConstructionScript`
  (set `self.isExplode` false)
  (`self.SetDamage` 15.0))