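; Player controller for the gem-collect mode that sets up the possessed tank pawn and releases it on death.
; On possess it caches the pawn, hands it the UI instance and refreshes the health bar.
; Depending on the current weapon type, it either spawns and force-collects a projectile pickup, or clears inventory counts and restocks and equips one weapon type.
; Lives, respawn and player-removal logic is present but disconnected.
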(event `/Game/Blueprint/PlayerControllers/Interface_PC.PawnDied`
  (`KismetSystemLibrary.PrintString` "gemcollect DEATH" true true (struct :`R` 0.697051 :`G` 0.033717 :`B` 1.0 :`A` 1.0))
  (`self.UnPossess` self))

(event `self.ReceivePossess`
  (params (PossessedPawn :type "Pawn Object Reference"))
  (bind (_value _returnvalue) (`BlueprintMapLibrary.Map_Find` (`/Game/Blueprint/InventorySystem/BP_InventoryComponent.InventoryDictionary` (`/Game/Blueprint/TankPawns/BP_PlayerTankBase.InventoryComponent` (`self.P_PlayerCollectGem`))) "NewEnumerator1"))
  (`parent.ReceivePossess` PossessedPawn)
  ;[1 1 1] Set Pawn Ref
  (bind _asp_tank_collect_gem (cast `/Game/Blueprint/TankPawns/GemCollectPawns/P_TankCollectGem` PossessedPawn))
  (bind _output_get (set `self.P_PlayerCollectGem` _asp_tank_collect_gem))
  ;[1 1 1] Update UI
  (bind _output_get_2 (set `/Game/Blueprint/TankPawns/GemCollectPawns/P_TankCollectGem.In Game UIRef` (`self.UI_Inst`) _output_get))
  (message `/Game/Blueprint/EnemyMob/zombie/Interface_UI_Health.UpdateHealthBar` _output_get_2 (`/Game/Blueprint/TankPawns/BP_PlayerTankBase.Health` _asp_tank_collect_gem) 0.0)
  (if (`|EnumEquality` (`/Game/Blueprint/TankPawns/BP_PlayerTankBase.CurrentWeaponType` (`self.P_PlayerCollectGem`)) "NewEnumerator4")
    (bind _returnvalue_2 (`|SpawnActorFromClass` "/Game/Blueprint/WeaponPickUp/BP_PickUpProjectile.BP_PickUpProjectile_C" (`self.GetTransform` (`self.P_PlayerCollectGem`)) "Undefined" "OverrideRootScale" null null))
    (`/Game/Blueprint/WeaponPickUp/BP_PickUpBase.DestroyPrePickupRefs` _returnvalue_2 (`self.P_PlayerCollectGem`))
    (`/Game/Blueprint/TankPawns/BP_PlayerTankBase.On Weapon Pick Up` (`self.P_PlayerCollectGem`) _returnvalue_2)
    (else
      (bind _values (`BlueprintMapLibrary.Map_Values` (`/Game/Blueprint/InventorySystem/BP_InventoryComponent.InventoryDictionary` (`/Game/Blueprint/TankPawns/BP_PlayerTankBase.InventoryComponent` (`self.P_PlayerCollectGem`)))))
      (for _array_element _values
        (set `/Game/Blueprint/InventorySystem/BP_InventorySlot.ItemCount` 0 _array_element)
        (if _returnvalue
          (set `/Game/Blueprint/InventorySystem/BP_InventorySlot.ItemCount` 30 _value)
          (message `/Game/Blueprint/PlayerInterface.ChangeToWeapon` (`self.P_PlayerCollectGem`) "NewEnumerator1"))))))

(fn `UserConstructionScript`)