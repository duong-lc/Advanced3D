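; Player controller for a sandbox tank game, handling tank movement, mouse-cursor turret aiming, weapons and ability swaps.
; Axis input feeds the movement component and a timeline that lerps the body toward its travel direction.
; Fire dispatches on the current weapon (machine-gun trace, projectile, mortar, orbital rocket), gated by pawn cooldowns and consuming inventory ammo, auto-switching when empty.
; Mouse wheel cycles weapons; SetAbility spawns and possesses a replacement pawn, destroying the old one.
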(event `self.ReceiveBeginPlay`
  ;[0.2266 0.427 1 1 50] Begin Play
  (`|ExecutionSequence`
    (:`then_0`
      (`self.InitReferencePawn` (`GameplayStatics.GetPlayerPawn` 0)))))

(event `self.ReceiveTick`
  (params (DeltaSeconds :type "Float (single-precision)"))
  (bind (_returnvalue_roll _returnvalue_pitch _returnvalue_yaw) (`KismetMathLibrary.BreakRotator` (`KismetMathLibrary.FindLookAtRotation` (`self.K2_GetActorLocation` (`self.K2_GetPawn`)) (`.Location` (`GameplayStatics.BreakHitResult` (`self.GetHitResultUnderCursorByChannel` (`GameplayStatics.GetPlayerController` 0) "TraceTypeQuery1" true))))))
  (bind _returnvalue (+ (+ (* (`self.GetActorForwardVector` (`self.PlayerPawn`)) (* (`self.fwdAxisVal`) 100.0)) (* (`self.GetActorRightVector` (`self.PlayerPawn`)) (* (`self.rightAxisVal`) 100.0))) (`self.K2_GetActorLocation` (`self.PlayerPawn`))))
  (bind (_returnvalue_roll_2 _returnvalue_pitch_2 _returnvalue_yaw_2) (`KismetMathLibrary.BreakRotator` (`KismetMathLibrary.FindLookAtRotation` (`SceneComponent.K2_GetComponentLocation` (`self.Body`)) _returnvalue)))
  (bind _returnvalue_2 (`KismetMathLibrary.MakeRotator` _returnvalue_roll_2 0.0 (+ _returnvalue_yaw_2 180.0)))
  ;[0.2699 0.4876 1 1 36] Tick
  (`SceneComponent.K2_SetWorldRotation` (`self.Turret`) (`KismetMathLibrary.MakeRotator` 0.0 0.0 _returnvalue_yaw) false false)
  (`KismetSystemLibrary.DrawDebugLine` (`self.K2_GetActorLocation` (`self.PlayerPawn`)) _returnvalue (struct :`G` 1.0 :`B` 0.103821 :`A` 1.0) 0.0 1.0)
  ;;[1 1 1] If there's input, update the rotation
  (if (or (!= (`self.rightAxisVal`) 0.0) (!= (`self.fwdAxisVal`) 0.0))
    ;;[1 1 1] Check if it's the same rotator with tolerance
    (if (not (== _returnvalue_2 (`self.currBodyRotation`) :`ErrorTolerance` 0.1))
      (set `self.currBodyRotation` _returnvalue_2))))

(event `self.ReceiveAnyDamage`
  (params (Damage :type "Float (single-precision)") (DamageType :type "DamageType Object Reference") (InstigatedBy :type "Controller Object Reference") (DamageCauser :type "Actor Object Reference"))
  (`/Game/Blueprint/TankPawns/BP_PlayerTankBase.TakeDamage` (`self.playerTank`) Damage))

(event `InputAxis|MoveRight`
  (params (AxisValue :type "Float (single-precision)"))
  ;[1 0.1779 0.484 1 36] Movement
  (set `self.rightAxisVal` AxisValue)
  (`PawnMovementComponent.AddInputVector` (`self.playerMovementCompo`) (`self.Get RightVelocity`) false)
  (bind (_direction _alphalerp) (`Timeline|LerpRotation` :!via `PlayFromStart` :!label _label)
    (:`Update`
      (`SceneComponent.K2_SetWorldRotation` (`self.Body`) (`KismetMathLibrary.RLerp` (`SceneComponent.K2_GetComponentRotation` (`self.Body`)) (`self.currBodyRotation`) _alphalerp true) false false))))

(event `Key|H`
  (params (Key :type "Key Structure"))
  (:`Pressed`
    (`GameplayStatics.ApplyDamage` (`GameplayStatics.GetPlayerController` 0) 10.0)))

(event `InputAxis|MoveForward`
  (params (AxisValue :type "Float (single-precision)"))
  ;[1 0.1779 0.484 1 36] Movement
  (set `self.fwdAxisVal` AxisValue)
  (`PawnMovementComponent.AddInputVector` (`self.playerMovementCompo`) (`self.Get Fwd Velocity`) false)
  (goto _label :!via `PlayFromStart`))

(event `InputAction|Fire`
  (params (Key :type "Key Structure"))
  (bind (_turret _world_location _world_rotation) (`self.BarrelTipLoc/Rot`))
  (bind (_turret_2 _world_location_2 _world_rotation_2) (`self.BarrelTipLoc/Rot`))
  ;[0.2465 1 0.9303 1 40] Combat
  (:`Pressed`
    (set `self.isHoldingFire` true)
    (switch `/Game/Blueprint/Enums/EnumWeaponType` (`self.currWeapon`)
      (:`NewEnumerator0`
        (if (`self.isHoldingFire`) :!label _label_2
          (`self.InitiateCurrentCoolDown`)
          (`self.RemoveItem`)
          (bind (_out_hit_impact_point _returnvalue) (`self.Fire_RayCast` 0.0 0.0))
          (if _returnvalue
            (`GameplayStatics.SpawnEmitterAtLocation` "/Game/Assets/Particles/BasicMachineGunHitPAR.BasicMachineGunHitPAR" _out_hit_impact_point (`KismetMathLibrary.FindLookAtRotation` (`.world location` (`self.BarrelTipLoc/Rot`)) _out_hit_impact_point) (2.0 2.0 2.0)))
          (if (`self.isHoldingFire`) :!label _label_3
            (bind _canshoot (`self.IsCoolDownComplete`))
            (if _canshoot
              (goto _label_2)
              (else
                (`KismetSystemLibrary.DelayUntilNextTick`)
                (goto _label_3))))))
      (:`NewEnumerator1`
        (bind _canshoot_2 (`self.IsCoolDownComplete`))
        (if _canshoot_2
          (`self.RemoveItem`)
          (bind _returnvalue_2 (`|SpawnActorFromClass` "/Game/Blueprint/Projectiles/BP_TankBullet.BP_TankBullet_C" (`KismetMathLibrary.MakeTransform` _world_location_2 _world_rotation_2) "Undefined" "OverrideRootScale" null null))
          (`/Engine/EditorBlueprintResources/StandardMacros.IsValid` _returnvalue_2
            (:`Is Valid`
              (set `/Game/Blueprint/Projectiles/BP_TankBullet.damage` 0.0 _returnvalue_2)
              (`/Game/Blueprint/Projectiles/BP_TankBullet.BulletTraverse` _returnvalue_2 (* 0.0 1.0))
              (`self.InitiateCurrentCoolDown`)))))
      (:`NewEnumerator2`
        (bind _canshoot_3 (`self.IsCoolDownComplete`))
        (if _canshoot_3
          (`self.RemoveItem`)
          (bind (_startpos _endpos) (`self.Fire_Mortar`))
          (bind _returnvalue_3 (`|SpawnActorFromClass` "/Game/Blueprint/Projectiles/BP_MortarRound.BP_MortarRound_C" (`KismetMathLibrary.MakeTransform` _world_location _world_rotation) "Undefined" "OverrideRootScale" null null))
          (`/Game/Blueprint/Projectiles/BP_MortarRound.OnSpawn` _returnvalue_3 _startpos _endpos)
          (`/Game/Blueprint/Projectiles/BP_MortarRound.SetDamage` _returnvalue_3 50.0)
          (`self.InitiateCurrentCoolDown`)))
      (:`NewEnumerator3`
        (bind _canshoot_4 (`self.IsCoolDownComplete`))
        (if _canshoot_4
          (`self.RemoveItem`)
          (bind (_start _end _rocketobj) (`self.Fire_OrbitalStrike`))
          (`/Game/Blueprint/Projectiles/BP_Rocket.SetDamage` _rocketobj 0.0)
          (`/Game/Blueprint/Projectiles/BP_Rocket.TraverseRocket` _rocketobj _start _end)
          (`self.InitiateCurrentCoolDown`)))))
  (:`Released`
    (set `self.isHoldingFire` false)
    (goto _label_2)))

(event `SetAbility`
  (params (`new Ability` :type "/Game/Blueprint/Enums/EnumAbilityType Enum" :default "NewEnumerator0"))
  ;[1 0.9465 0.2199 1 40] Ability
  (`KismetSystemLibrary.DelayUntilNextTick`)
  (bind _output_get (set `self.currAbilityMode` `new Ability`))
  (bind _returnvalue (`|SpawnActorFromClass` (`BlueprintMapLibrary.Map_Find` (`self.pawnDict`) _output_get) (`self.GetTransform` (`GameplayStatics.GetPlayerPawn` 0)) "Undefined" "OverrideRootScale" null null))
  (`self.UnPossess`)
  (`self.Possess` _returnvalue))

(event `Key|MouseScrollUp`
  (params (Key :type "Key Structure"))
  ;[0.8325 0.2617 1 1 40] Weapon Slot
  ;;[1 1 1] Switch to Previous Slot
  (:`Pressed`
    (bind (_slot _previous_weapon_enum _shouldcycle) (`/Game/Blueprint/InventorySystem/BP_InventoryComponent.GetPreviousItem` (`/Game/Blueprint/TankPawns/BP_PlayerTankBase.InventoryComponent` (`self.playerTank`)) (`self.currWeapon`)))
    (if _shouldcycle
      (`self.SetCurrentWeapon` _previous_weapon_enum (`/Game/Blueprint/InventorySystem/BP_InventorySlot.PickUpRef` _slot)))))

(event `self.ReceivePossess`
  (params (PossessedPawn :type "Pawn Object Reference"))
  ;[1 0.9465 0.2199 1 40] Ability
  (`self.InitReferencePawn` PossessedPawn))

(event `Key|MouseScrollDown`
  (params (Key :type "Key Structure"))
  ;[0.8325 0.2617 1 1 40] Weapon Slot
  ;;[1 1 1] Switch to Next Slot
  (:`Pressed`
    (bind (_slot _next_weapon_enum _shouldcycle) (`/Game/Blueprint/InventorySystem/BP_InventoryComponent.Get Next Item` (`/Game/Blueprint/TankPawns/BP_PlayerTankBase.InventoryComponent` (`self.playerTank`)) (`self.currWeapon`)))
    (if _shouldcycle
      (`self.SetCurrentWeapon` _next_weapon_enum (`/Game/Blueprint/InventorySystem/BP_InventorySlot.PickUpRef` _slot)))))

(event `self.ReceiveUnPossess`
  (params (UnpossessedPawn :type "Pawn Object Reference"))
  ;[1 0.9465 0.2199 1 40] Ability
  (`self.K2_DestroyActor` UnpossessedPawn))

(fn `Ability_Activate`
  (params (Scale :type "Vector Structure") (maxHealth :type "Float (double-precision)") (speed :type "Float (double-precision)") (Material :type "MaterialInterface Object Reference"))
  (locals (mat :type "MaterialInterface Object Reference") (scaleToSet :type "Vector Structure") (maxHealthToSet :type "Float (double-precision)") (speedToSet :type "Float (double-precision)"))
  (`|ExecutionSequence`
    (:`then_0`
      (set `local.scaleToSet` Scale))
    (:`then_1`
      (set `local.maxHealthToSet` maxHealth))
    (:`then_2`
      (set `local.speedToSet` speed))
    (:`then_3`
      (set `local.mat` Material))
    (:`then_4`
      (`|ExecutionSequence`
        (:`then_0`
          ;[1 1 1] Set Tank Scale
          (`SceneComponent.SetWorldScale3D` (`/Game/Blueprint/TankPawns/BP_PlayerTankBase.Body` (`self.playerTank`)) (`local.scaleToSet`)))
        (:`then_1`
          ;[1 1 1] Set Health and max Health
          (bind _output_get (set `/Game/Blueprint/TankPawns/BP_PlayerTankBase.maxHealth` (`local.maxHealthToSet`) (`self.playerTank`)))
          (set `/Game/Blueprint/TankPawns/BP_PlayerTankBase.Health` _output_get (`self.playerTank`)))
        (:`then_2`
          ;[1 1 1] Set Speed
          (set `/Game/Blueprint/TankPawns/BP_PlayerTankBase.speed` (`local.speedToSet`) (`self.playerTank`)))
        (:`then_3`
          ;[1 1 1] Set Material
          (`PrimitiveComponent.SetMaterial` (`/Game/Blueprint/TankPawns/BP_PlayerTankBase.Body` (`self.playerTank`)) 0 (`local.mat`)))
        (:`then_4`
          (switch `/Game/Blueprint/Enums/EnumAbilityType` (`self.currAbilityMode`)
            (:`NewEnumerator0`
              (`PrimitiveComponent.SetMaterial` (`/Game/Blueprint/TankPawns/BP_PlayerTankBase.Body` (`self.playerTank`)) 1 "/Game/Assets/EnemyMesh/En_Mat02.En_Mat02" :!label _label))
            (:`NewEnumerator1`
              (goto _label))
            (:`NewEnumerator2`
              (goto _label))
            (:`NewEnumerator3`
              (`PrimitiveComponent.SetMaterial` (`/Game/Blueprint/TankPawns/BP_PlayerTankBase.Body` (`self.playerTank`)) 1 "/Game/Assets/EnemyMesh/AlphaMat.AlphaMat"))))))))

(fn `Fire_Mortar`
  (returns (startPos :type "Vector Structure") (endPos :type "Vector Structure"))
  (locals (endLocation :type "Vector Structure" :default (0.0 0.0 0.0)) (startLocation :type "Vector Structure" :default (0.0 0.0 0.0)))
  (bind _output_get (set `local.startLocation` (`SceneComponent.GetSocketLocation` (`self.Turret`) "barrelTip")))
  (bind _output_get_2 (set `local.endLocation` (`.Location` (`GameplayStatics.BreakHitResult` (`self.GetHitResultUnderCursorByChannel` (`GameplayStatics.GetPlayerController` 0) "TraceTypeQuery1" true)))))
  (return _output_get _output_get_2))

(fn `Fire_OrbitalStrike`
  (returns (start :type "Vector Structure") (end :type "Vector Structure") (rocketObj :type "/Game/Blueprint/Projectiles/BP_Rocket Object Reference"))
  (locals (endPos :type "Vector Structure" :default (0.0 0.0 0.0)) (startPos :type "Vector Structure"))
  ;[1 1 1] Setting end position as the position of the mouse click into the world
  (bind _output_get (set `local.endPos` (`.Location` (`GameplayStatics.BreakHitResult` (`self.GetHitResultUnderCursorByChannel` (`GameplayStatics.GetPlayerController` 0) "TraceTypeQuery1" true)))))
  ;[1 1 1] Start position is just end position with height offset
  (bind _output_get_2 (set `local.startPos` (+ _output_get (0.0 0.0 600.0))))
  (bind _returnvalue (`|SpawnActorFromClass` "/Game/Blueprint/Projectiles/BP_Rocket.BP_Rocket_C" (`KismetMathLibrary.MakeTransform` _output_get_2) "Undefined" "OverrideRootScale" null null :!pinned true)) ; Spawn Rocket blueprint actor
  (return _output_get_2 _output_get _returnvalue))

(fn `Fire_Projectile`
  (params (Force :type "Float (single-precision)") (damage :type "Float (double-precision)") (cooldown :type "Float (double-precision)")))

(fn `Fire_RayCast`
  (params (`Ray cast Range` :type "Float (single-precision)") (damage :type "Float (double-precision)"))
  (returns (`Out Hit Impact Point` :type "Vector Structure") (ReturnValue :type Boolean))
  (bind (_end _start) (`self.GetRayCastEssentials` `Ray cast Range`))
  (`GameplayStatics.SpawnEmitterAtLocation` "/Game/Assets/Particles/BasicMachineGunFirePAR.BasicMachineGunFirePAR" _start (`KismetMathLibrary.FindLookAtRotation` _start _end) (1.5 1.5 1.5))
  (bind (_outhit _returnvalue) (`KismetSystemLibrary.LineTraceSingle` _start _end "TraceTypeQuery1" false (`self.Actors to Ignore`)))
  (`GameplayStatics.ApplyDamage` (`.HitActor` (`GameplayStatics.BreakHitResult` _outhit)) damage)
  (return (`.ImpactPoint` (`GameplayStatics.BreakHitResult` _outhit)) _returnvalue))

(fn `Get Fwd Velocity`
  (returns (`Local Forward Vector` :type "Vector Structure"))
  (return (* (`self.GetActorForwardVector` (`self.PlayerPawn`)) (* (`self.fwdAxisVal`) (`/Game/Blueprint/TankPawns/BP_PlayerTankBase.speed` (`self.playerTank`))))))

(fn `Get RightVelocity`
  (returns (`Local Right Vector` :type "Vector Structure"))
  (return (* (`self.GetActorRightVector` (`self.PlayerPawn`)) (* (`self.rightAxisVal`) (`/Game/Blueprint/TankPawns/BP_PlayerTankBase.speed` (`self.playerTank`))))))

(fn `GetRayCastEssentials`
  (params (`Ray cast Range` :type "Float (single-precision)"))
  (returns (End :type "Vector Structure") (Start :type "Vector Structure"))
  (return (+ (`.world location` (`self.BarrelTipLoc/Rot`)) (* (`KismetMathLibrary.GetForwardVector` (`SceneComponent.K2_GetComponentRotation` (`self.BarrelTipLoc/Rot`))) (`KismetMathLibrary.Conv_DoubleToVector` `Ray cast Range`))) (`.world location` (`self.BarrelTipLoc/Rot`))))

(fn `InitReferencePawn`
  (params (PlayerPawn :type "Pawn Object Reference"))
  (set `self.PlayerPawn` PlayerPawn)
  ;[1 1 1] Cast to get BP class and set up components
  (bind _asbp_player_tank_base (cast `/Game/Blueprint/TankPawns/BP_PlayerTankBase` (`self.PlayerPawn`)))
  (bind _output_get (set `self.playerTank` _asbp_player_tank_base))
  (set `self.Body` (`/Game/Blueprint/TankPawns/BP_PlayerTankBase.Body` _output_get))
  (set `self.playerMovementCompo` (`Pawn.GetMovementComponent` (`self.PlayerPawn`))))

(fn `IsCoolDownComplete`
  (returns (canShoot :type Boolean) (coolDown :type "Float (double-precision)"))
  (bind (_canshoot _cooldown) (message `/Game/Blueprint/PlayerInterface.ReturnCurrentCoolDown` (`self.PlayerPawn`)))
  (return _canshoot _cooldown))

(fn `SetCurrentWeapon`
  (params (currWeapon :type "/Game/Blueprint/Enums/EnumWeaponType Enum" :default "NewEnumerator4") (weapon :type "/Game/Blueprint/WeaponPickUp/BP_PickUpBase Object Reference"))
  (set `self.currWeapon` currWeapon)
  (`/Game/Blueprint/TankPawns/BP_PlayerTankBase.OnWeaponChange` (`self.playerTank`) weapon))

(fn `UserConstructionScript`
  (`KismetArrayLibrary.Array_AddUnique` (`self.Actors to Ignore`) (`self.K2_GetPawn`)))