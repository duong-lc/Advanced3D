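; Player controller for the Turf War tank mode that tracks a player's lives and links the tank to the in-game UI.
; On possess, it refreshes health and lives displays, then either gives a spawned projectile pickup or resets inventory counts to a default weapon loadout, depending on current weapon type.
; On pawn death, it decrements lives and unpossesses for respawn, or removes the player when none remain.
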(event `/Game/Blueprint/PlayerControllers/Interface_PC.PawnDied`
  (`KismetSystemLibrary.PrintString` "TURF WAR DEATH" true true (struct :`R` 0.697051 :`G` 0.033717 :`B` 1.0 :`A` 1.0))
  ;[1 1 1] Removing a life
  (bind _result (`/Engine/EditorBlueprintResources/StandardMacros.DecrementInt` (`self.lives`))
    (:`  `
      (if (>= _result 1)
        ;[1 1 1] Respawning
        (cast `/Game/Blueprint/GameModes/GM_TurfWar` (`GameplayStatics.GetGameMode`))
        (message `/Game/Blueprint/EnemyMob/zombie/Interface_UI_Health.UpdateLives` (`self.UI_Inst`) (`self.lives`))
        (`self.UnPossess` self)
        (else
          ;[1 1 1] Out of life -> remove player
          (`GameplayStatics.RemovePlayer` self true))))))

(event `self.ReceivePossess`
  (params (PossessedPawn :type "Pawn Object Reference"))
  (bind _lives (`self.lives`))
  (bind (_value _returnvalue) (`BlueprintMapLibrary.Map_Find` (`/Game/Blueprint/InventorySystem/BP_InventoryComponent.InventoryDictionary` (`/Game/Blueprint/TankPawns/BP_PlayerTankBase.InventoryComponent` (`self.P_PlayerTurfWar`))) "NewEnumerator1"))
  (`parent.ReceivePossess` PossessedPawn)
  ;[1 1 1] Set Pawn Ref
  (bind _asp_tank_turf_war (cast `/Game/Blueprint/TankPawns/TurfWarPawns/P_TankTurfWar` PossessedPawn))
  (bind _output_get (set `self.P_PlayerTurfWar` _asp_tank_turf_war))
  ;[1 1 1] Update UI
  (bind _output_get_2 (set `/Game/Blueprint/TankPawns/TurfWarPawns/P_TankTurfWar.In Game UIRef` (`self.UI_Inst`) _output_get))
  (message `/Game/Blueprint/EnemyMob/zombie/Interface_UI_Health.UpdateHealthBar` _output_get_2 (`/Game/Blueprint/TankPawns/BP_PlayerTankBase.Health` _asp_tank_turf_war) (`/Game/Blueprint/TankPawns/BP_PlayerTankBase.maxHealth` _asp_tank_turf_war))
  (`KismetSystemLibrary.PrintString` (`KismetStringLibrary.Conv_IntToString` _lives) true true (struct :`R` 0.866855 :`G` 1.0 :`A` 1.0))
  (message `/Game/Blueprint/EnemyMob/zombie/Interface_UI_Health.UpdateLives` (`self.UI_Inst`) _lives)
  (if (`|EnumEquality` (`/Game/Blueprint/TankPawns/BP_PlayerTankBase.CurrentWeaponType` (`self.P_PlayerTurfWar`)) "NewEnumerator4")
    (bind _returnvalue_2 (`|SpawnActorFromClass` "/Game/Blueprint/WeaponPickUp/BP_PickUpProjectile.BP_PickUpProjectile_C" (`self.GetTransform` (`self.P_PlayerTurfWar`)) "Undefined" "OverrideRootScale" null null))
    (`/Game/Blueprint/WeaponPickUp/BP_PickUpBase.DestroyPrePickupRefs` _returnvalue_2 (`self.P_PlayerTurfWar`))
    (`/Game/Blueprint/TankPawns/BP_PlayerTankBase.On Weapon Pick Up` (`self.P_PlayerTurfWar`) _returnvalue_2)
    (else
      (bind _values (`BlueprintMapLibrary.Map_Values` (`/Game/Blueprint/InventorySystem/BP_InventoryComponent.InventoryDictionary` (`/Game/Blueprint/TankPawns/BP_PlayerTankBase.InventoryComponent` (`self.P_PlayerTurfWar`)))))
      (for _array_element _values
        (set `/Game/Blueprint/InventorySystem/BP_InventorySlot.ItemCount` 0 _array_element)
        (if _returnvalue
          (set `/Game/Blueprint/InventorySystem/BP_InventorySlot.ItemCount` 30 _value)
          (message `/Game/Blueprint/PlayerInterface.ChangeToWeapon` (`self.P_PlayerTurfWar`) "NewEnumerator1"))))))

(event `/Game/Blueprint/TurfWar/PC_TurfWarInterface.LinkUIRef`
  (params (TurfWarInGameUI :type "/Game/Blueprint/HUD/UI_InGame_TurfWar Object Reference"))
  (set `self.UI_Inst` TurfWarInGameUI))

(fn `GetUIRef`
  (returns (InGameUIRef :type "/Game/Blueprint/HUD/UI_InGame_TurfWar Object Reference"))
  (return null))

(fn `UserConstructionScript`)