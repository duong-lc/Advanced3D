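; Player controller for the capture-objective mode that drives a P_TankObjective pawn.
; On possess it hands the pawn the UI stored by LinkUIRef, updates the health bar and sets up the starting weapon.
; That setup either spawns and grants a pickup projectile or clears inventory counts, restocks one weapon and switches to it.
; PawnDied only unpossesses; the lives, respawn and player-removal logic is unconnected.
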(event `/Game/Blueprint/PlayerControllers/Interface_PC.PawnDied`
  (`KismetSystemLibrary.PrintString` "Objective DEATH" true true (struct :`R` 0.697051 :`G` 0.033717 :`B` 1.0 :`A` 1.0))
  (`self.UnPossess` self))

(event `self.ReceivePossess`
  (params (PossessedPawn :type "Pawn Object Reference"))
  (bind (_value _returnvalue) (`BlueprintMapLibrary.Map_Find` (`/Game/Blueprint/InventorySystem/BP_InventoryComponent.InventoryDictionary` (`/Game/Blueprint/TankPawns/BP_PlayerTankBase.InventoryComponent` (`self.P_PlayerObjective`))) "NewEnumerator1"))
  (`parent.ReceivePossess` PossessedPawn)
  ;[1 1 1] Set Pawn Ref
  (bind _asp_tank_objective (cast `/Game/Blueprint/TankPawns/CaptureObjectivePawns/P_TankObjective` PossessedPawn))
  (bind _output_get (set `self.P_PlayerObjective` _asp_tank_objective))
  ;[1 1 1] Update UI
  (bind _output_get_2 (set `/Game/Blueprint/TankPawns/CaptureObjectivePawns/P_TankObjective.In Game UIRef` (`self.UI_Inst`) _output_get))
  (message `/Game/Blueprint/EnemyMob/zombie/Interface_UI_Health.UpdateHealthBar` _output_get_2 (`/Game/Blueprint/TankPawns/BP_PlayerTankBase.Health` _asp_tank_objective) 0.0)
  (if (`|EnumEquality` (`/Game/Blueprint/TankPawns/BP_PlayerTankBase.CurrentWeaponType` (`self.P_PlayerObjective`)) "NewEnumerator4")
    (bind _returnvalue_2 (`|SpawnActorFromClass` "/Game/Blueprint/WeaponPickUp/BP_PickUpProjectile.BP_PickUpProjectile_C" (`self.GetTransform` (`self.P_PlayerObjective`)) "Undefined" "OverrideRootScale" null null))
    (`/Game/Blueprint/WeaponPickUp/BP_PickUpBase.DestroyPrePickupRefs` _returnvalue_2 (`self.P_PlayerObjective`))
    (`/Game/Blueprint/TankPawns/BP_PlayerTankBase.On Weapon Pick Up` (`self.P_PlayerObjective`) _returnvalue_2)
    (else
      (bind _values (`BlueprintMapLibrary.Map_Values` (`/Game/Blueprint/InventorySystem/BP_InventoryComponent.InventoryDictionary` (`/Game/Blueprint/TankPawns/BP_PlayerTankBase.InventoryComponent` (`self.P_PlayerObjective`)))))
      (for _array_element _values
        (set `/Game/Blueprint/InventorySystem/BP_InventorySlot.ItemCount` 0 _array_element)
        (if _returnvalue
          (set `/Game/Blueprint/InventorySystem/BP_InventorySlot.ItemCount` 30 _value)
          (message `/Game/Blueprint/PlayerInterface.ChangeToWeapon` (`self.P_PlayerObjective`) "NewEnumerator1"))))))

(event `/Game/Blueprint/PlayerControllers/PC_ObjectiveInterface.LinkUIRef`
  (params (`UI In Game` :type "/Game/Blueprint/CaptureObj/UI_InGameCaptureObj Object Reference"))
  (set `self.UI_Inst` `UI In Game`))

(fn `GetUIRef`
  (returns (`UI In Game` :type "/Game/Blueprint/CaptureObj/UI_InGameCaptureObj Object Reference"))
  (return null))

(fn `UserConstructionScript`)