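; Player controller for the DeathMatch tank mode, driving the possessed tank's movement, aiming, firing and lives.
; Axis input moves the tank while a timeline lerps its body toward the input direction; the current weapon follows the cursor or spins with arrow keys.
; Firing and mouse-wheel slot switching go through messages to the weapon and pawn.
; On death it decrements lives, then restarts the player or removes them when none remain.
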(event `self.ReceiveBeginPlay`
  ;[0.2266 0.427 1 1 50] Begin Play
  (`|ExecutionSequence`
    (:`then_0`
      (`self.InitReferencePawn` (`GameplayStatics.GetPlayerPawn` 0)))))

(event `self.ReceiveTick`
  (params (DeltaSeconds :type "Float (single-precision)"))
  (bind (_returnvalue_roll _returnvalue_pitch _returnvalue_yaw) (`KismetMathLibrary.BreakRotator` (`KismetMathLibrary.FindLookAtRotation` (`self.K2_GetActorLocation` (`self.K2_GetPawn`)) (`.Location` (`GameplayStatics.BreakHitResult` (`self.GetHitResultUnderCursorByChannel` (`GameplayStatics.GetPlayerController` 0) "TraceTypeQuery1" true))))))
  (bind _returnvalue (+ (+ (* (`self.GetActorForwardVector` (`self.PlayerPawn`)) (* (`self.fwdAxisVal`) 100.0)) (* (`self.GetActorRightVector` (`self.PlayerPawn`)) (* (`self.rightAxisVal`) 100.0))) (`self.K2_GetActorLocation` (`self.PlayerPawn`))))
  (bind (_returnvalue_roll_2 _returnvalue_pitch_2 _returnvalue_yaw_2) (`KismetMathLibrary.BreakRotator` (`KismetMathLibrary.FindLookAtRotation` (`SceneComponent.K2_GetComponentLocation` (`self.Body`)) _returnvalue)))
  (bind _returnvalue_2 (`KismetMathLibrary.MakeRotator` _returnvalue_roll_2 0.0 (+ _returnvalue_yaw_2 180.0)))
  ;[0.2699 0.4876 1 1 36] Tick
  (bind _weapontype (`self.GetCurrentWeaponType`))
  (bind (_weapon_ref _isfound) (`/Game/Blueprint/TankPawns/BP_PlayerTankBase.GetCurrentWeapon` (`self.playerTank`) _weapontype))
  (if _isfound
    (`SceneComponent.K2_SetWorldRotation` (`Actor.RootComponent` _weapon_ref) (`KismetMathLibrary.MakeRotator` 0.0 0.0 _returnvalue_yaw) false false))
  (`KismetSystemLibrary.DrawDebugLine` (`self.K2_GetActorLocation` (`self.PlayerPawn`)) _returnvalue (struct :`G` 1.0 :`B` 0.103821 :`A` 1.0) 0.0 1.0)
  ;;[1 1 1] If there's input, update the rotation
  (if (or (!= (`self.rightAxisVal`) 0.0) (!= (`self.fwdAxisVal`) 0.0))
    ;;[1 1 1] Check if it's the same rotator with tolerance
    (if (not (== _returnvalue_2 (`self.currBodyRotation`) :`ErrorTolerance` 0.1))
      (set `self.currBodyRotation` _returnvalue_2))))

(event `Key|Left`
  (params (Key :type "Key Structure"))
  (:`Pressed`
    (set `self.spinLeft` true)
    (if (`self.spinLeft`) :!label _label
      (bind _weapontype (`self.GetCurrentWeaponType`))
      (bind (_weapon_ref _isfound) (`/Game/Blueprint/TankPawns/BP_PlayerTankBase.GetCurrentWeapon` (`self.playerTank`) _weapontype))
      (if _isfound
        (`self.K2_AddActorLocalRotation` _weapon_ref (struct :`Yaw` -2.5) false false)
        (`KismetSystemLibrary.DelayUntilNextTick`)
        (goto _label))))
  (:`Released`
    (set `self.spinLeft` false)))

(event `InputAxis|MoveRight`
  (params (AxisValue :type "Float (single-precision)"))
  (bind _body (`self.Body`))
  ;[1 0.1779 0.484 1 36] Movement
  (set `self.rightAxisVal` AxisValue)
  (`PawnMovementComponent.AddInputVector` (`self.playerMovementCompo`) (`self.Get RightVelocity`) false)
  (bind (_direction _alphalerp) (`Timeline|LerpRotation` :!via `PlayFromStart` :!label _label_2)
    (:`Update`
      (`/Engine/EditorBlueprintResources/StandardMacros.IsValid` _body
        (:`Is Valid`
          (`SceneComponent.K2_SetWorldRotation` _body (`KismetMathLibrary.RLerp` (`SceneComponent.K2_GetComponentRotation` (`self.Body`)) (`self.currBodyRotation`) _alphalerp true) false false))))))

(event `Key|Right`
  (params (Key :type "Key Structure"))
  (:`Pressed`
    (set `self.spinRight` true)
    (if (`self.spinRight`) :!label _label_3
      (bind _weapontype (`self.GetCurrentWeaponType`))
      (bind (_weapon_ref _isfound) (`/Game/Blueprint/TankPawns/BP_PlayerTankBase.GetCurrentWeapon` (`self.playerTank`) _weapontype))
      (if _isfound
        (`self.K2_AddActorLocalRotation` _weapon_ref (struct :`Yaw` 2.5) false false)
        (`KismetSystemLibrary.DelayUntilNextTick`)
        (goto _label_3))))
  (:`Released`
    (set `self.spinRight` false)))

(event `InputAxis|MoveForward`
  (params (AxisValue :type "Float (single-precision)"))
  ;[1 0.1779 0.484 1 36] Movement
  (set `self.fwdAxisVal` AxisValue)
  (`PawnMovementComponent.AddInputVector` (`self.playerMovementCompo`) (`self.Get Fwd Velocity`) false)
  (goto _label_2 :!via `PlayFromStart`))

(event `InputAction|Fire`
  (params (Key :type "Key Structure"))
  ;[0.2819 0.7132 1 1 40] Combat
  (:`Pressed`
    (bind _weapontype (`self.GetCurrentWeaponType`))
    (switch `/Game/Blueprint/Enums/EnumWeaponType` _weapontype
      (:`NewEnumerator0`
        (set `self.isHoldingFire` true)
        (`self.FireWeapon` :!label _label_4))
      (:`NewEnumerator1`
        (`self.FireWeapon`))
      (:`NewEnumerator2`
        (`self.FireWeapon`))
      (:`NewEnumerator3`
        (`self.FireWeapon`))))
  (:`Released`
    (bind _weapontype_2 (`self.GetCurrentWeaponType`))
    (switch `/Game/Blueprint/Enums/EnumWeaponType` _weapontype_2
      (:`NewEnumerator0`
        (set `self.isHoldingFire` false)
        (goto _label_4)))))

(event `SetAbility`
  (params (`new Ability` :type "/Game/Blueprint/Enums/EnumAbilityType Enum" :default "NewEnumerator0"))
  ;[1 0.9465 0.2199 1 40] Ability
  (`KismetSystemLibrary.DelayUntilNextTick`))

(event `Key|MouseScrollUp`
  (params (Key :type "Key Structure"))
  ;[0.8325 0.2617 1 1 40] Weapon Slot
  ;;[1 1 1] Switch to Previous Slot
  (:`Pressed`
    (message `/Game/Blueprint/PlayerInterface.ChangeToPrevWeapon` (`self.PlayerPawn`))))

(event `self.ReceivePossess`
  (params (PossessedPawn :type "Pawn Object Reference"))
  ;[1 0.9465 0.2199 1 40] Ability
  (`self.InitReferencePawn` PossessedPawn))

(event `Key|MouseScrollDown`
  (params (Key :type "Key Structure"))
  ;[0.8325 0.2617 1 1 40] Weapon Slot
  ;;[1 1 1] Switch to Next Slot
  (:`Pressed`
    (message `/Game/Blueprint/PlayerInterface.ChangeToNextWeapon` (`self.PlayerPawn`))))

(event `self.ReceiveUnPossess`
  (params (UnpossessedPawn :type "Pawn Object Reference"))
  ;[1 0.9465 0.2199 1 40] Ability
  (`self.K2_DestroyActor` UnpossessedPawn))

(event `/Game/Blueprint/PlayerControllers/Interface_PC.OnWeaponChange`
  (set `self.isHoldingFire` false))

(event `/Game/Blueprint/PlayerControllers/Interface_PC.PawnDied`
  (bind _result (`/Engine/EditorBlueprintResources/StandardMacros.DecrementInt` (`self.lives`))
    (:`  `
      (if (>= _result 1)
        (`KismetSystemLibrary.Delay` 1.0)
        (while (not (`KismetSystemLibrary.IsValid` (`self.K2_GetPawn`)))
          (`GameModeBase.RestartPlayer` (`GameplayStatics.GetGameMode`) self))
        (else
          (`GameplayStatics.RemovePlayer` self true))))))

(fn `Ability_Activate`
  (params (Scale :type "Vector Structure") (maxHealth :type "Float (double-precision)") (speed :type "Float (double-precision)") (Material :type "MaterialInterface Object Reference"))
  (locals (mat :type "MaterialInterface Object Reference") (scaleToSet :type "Vector Structure") (maxHealthToSet :type "Float (double-precision)") (speedToSet :type "Float (double-precision)"))
  (`|ExecutionSequence`
    (:`then_0`
      (set `local.scaleToSet` Scale))
    (:`then_1`
      (set `local.maxHealthToSet` maxHealth))
    (:`then_2`
      (set `local.speedToSet` speed))
    (:`then_3`
      (set `local.mat` Material))
    (:`then_4`
      (`|ExecutionSequence`
        (:`then_0`
          ;[1 1 1] Set Tank Scale
          (`SceneComponent.SetWorldScale3D` (`/Game/Blueprint/TankPawns/BP_PlayerTankBase.Body` (`self.playerTank`)) (`local.scaleToSet`)))
        (:`then_1`
          ;[1 1 1] Set Health and max Health
          (bind _output_get (set `/Game/Blueprint/TankPawns/BP_PlayerTankBase.maxHealth` (`local.maxHealthToSet`) (`self.playerTank`)))
          (set `/Game/Blueprint/TankPawns/BP_PlayerTankBase.Health` _output_get (`self.playerTank`)))
        (:`then_2`
          ;[1 1 1] Set Speed
          (set `/Game/Blueprint/TankPawns/BP_PlayerTankBase.speed` (`local.speedToSet`) (`self.playerTank`)))
        (:`then_3`
          ;[1 1 1] Set Material
          (`PrimitiveComponent.SetMaterial` (`/Game/Blueprint/TankPawns/BP_PlayerTankBase.Body` (`self.playerTank`)) 0 (`local.mat`)))
        (:`then_4`
          (switch `/Game/Blueprint/Enums/EnumAbilityType` "NewEnumerator0"
            (:`NewEnumerator0`
              (`PrimitiveComponent.SetMaterial` (`/Game/Blueprint/TankPawns/BP_PlayerTankBase.Body` (`self.playerTank`)) 1 "/Game/Assets/EnemyMesh/En_Mat02.En_Mat02" :!label _label))
            (:`NewEnumerator1`
              (goto _label))
            (:`NewEnumerator2`
              (goto _label))
            (:`NewEnumerator3`
              (`PrimitiveComponent.SetMaterial` (`/Game/Blueprint/TankPawns/BP_PlayerTankBase.Body` (`self.playerTank`)) 1 "/Game/Assets/EnemyMesh/AlphaMat.AlphaMat"))))))))

(fn `AmmoDecrement`
  (returns (isSlotEmpty :type Boolean))
  (bind _weapontype (`self.GetCurrentWeaponType`))
  ;[1 1 1] Removing an ammo count in inventory according to current weapon's enum.
  (bind _isslotempty (`/Game/Blueprint/InventorySystem/BP_InventoryComponent.RemoveItem` (`/Game/Blueprint/TankPawns/BP_PlayerTankBase.InventoryComponent` (`self.playerTank`)) _weapontype))
  ;[1 1 1] Check if current slot is empty
  (if _isslotempty
    ;[1 1 1] Getting next available slot in inventory
    (bind (_newcurrenum _newcurriventoryslot _canget) (`/Game/Blueprint/InventorySystem/BP_InventoryComponent.GetNextAvailable` (`/Game/Blueprint/TankPawns/BP_PlayerTankBase.InventoryComponent` (`self.playerTank`))))
    (`KismetSystemLibrary.PrintString` (`KismetStringLibrary.Concat_StrStr` (`|GetEnumeratorNameAsString` _newcurrenum) " weapon type lol"))
    ;[1 1 1] Check If "Next Available Slot" was able to get to, if it is, set that as current weapon, if not, then ignore getting and setting to next available slot
    (if _canget
      (message `/Game/Blueprint/PlayerInterface.ChangeToWeapon` (`self.playerTank`) _newcurrenum)))
  (return _isslotempty))

(fn `AmmoUsed`
  (returns (`is Slot Empty` :type Boolean))
  (bind _isslotempty (`self.AmmoDecrement`))
  (return _isslotempty))

(fn `Fire_Mortar`
  (returns (startPos :type "Vector Structure") (endPos :type "Vector Structure"))
  (locals (endLocation :type "Vector Structure" :default (0.0 0.0 0.0)) (startLocation :type "Vector Structure" :default (0.0 0.0 0.0)))
  (bind _output_get (set `local.startLocation` (`SceneComponent.GetSocketLocation` (`self.Turret`) "barrelTip")))
  (bind _output_get_2 (set `local.endLocation` (`.Location` (`GameplayStatics.BreakHitResult` (`self.GetHitResultUnderCursorByChannel` (`GameplayStatics.GetPlayerController` 0) "TraceTypeQuery1" true)))))
  (return _output_get _output_get_2))

(fn `Fire_OrbitalStrike`
  (returns (start :type "Vector Structure") (end :type "Vector Structure") (rocketObj :type "/Game/Blueprint/Projectiles/BP_Rocket Object Reference"))
  (locals (endPos :type "Vector Structure" :default (0.0 0.0 0.0)) (startPos :type "Vector Structure"))
  ;[1 1 1] Setting end position as the position of the mouse click into the world
  (bind _output_get (set `local.endPos` (`.Location` (`GameplayStatics.BreakHitResult` (`self.GetHitResultUnderCursorByChannel` (`GameplayStatics.GetPlayerController` 0) "TraceTypeQuery1" true)))))
  ;[1 1 1] Start position is just end position with height offset
  (bind _output_get_2 (set `local.startPos` (+ _output_get (0.0 0.0 600.0))))
  (bind _returnvalue (`|SpawnActorFromClass` "/Game/Blueprint/Projectiles/BP_Rocket.BP_Rocket_C" (`KismetMathLibrary.MakeTransform` _output_get_2) "Undefined" "OverrideRootScale" null null :!pinned true)) ; Spawn Rocket blueprint actor
  (return _output_get_2 _output_get _returnvalue))

(fn `Fire_Projectile`
  (params (Force :type "Float (single-precision)") (damage :type "Float (double-precision)") (cooldown :type "Float (double-precision)")))

(fn `Fire_RayCast`
  (params (`Ray cast Range` :type "Float (single-precision)") (damage :type "Float (double-precision)"))
  (returns (`Out Hit Impact Point` :type "Vector Structure") (ReturnValue :type Boolean))
  (bind (_end _start) (`self.GetRayCastEssentials` `Ray cast Range`))
  (`GameplayStatics.SpawnEmitterAtLocation` "/Game/Assets/Particles/BasicMachineGunFirePAR.BasicMachineGunFirePAR" _start (`KismetMathLibrary.FindLookAtRotation` _start _end) (1.5 1.5 1.5))
  (bind (_outhit _returnvalue) (`KismetSystemLibrary.LineTraceSingle` _start _end "TraceTypeQuery1" false (`self.Actors to Ignore`)))
  (`GameplayStatics.ApplyDamage` (`.HitActor` (`GameplayStatics.BreakHitResult` _outhit)) damage)
  (return (`.ImpactPoint` (`GameplayStatics.BreakHitResult` _outhit)) _returnvalue))

(fn `Get Fwd Velocity`
  (returns (`Local Forward Vector` :type "Vector Structure"))
  (bind _playertank (`self.playerTank`))
  (`/Engine/EditorBlueprintResources/StandardMacros.IsValid` _playertank
    (:`Is Valid`
      (return (* (`self.GetActorForwardVector` _playertank) (* (`self.fwdAxisVal`) (`/Game/Blueprint/TankPawns/BP_PlayerTankBase.speed` _playertank)))))))

(fn `Get RightVelocity`
  (returns (`Local Right Vector` :type "Vector Structure"))
  (bind _playertank (`self.playerTank`))
  (`/Engine/EditorBlueprintResources/StandardMacros.IsValid` _playertank
    (:`Is Valid`
      (return (* (`self.GetActorRightVector` _playertank) (* (`self.rightAxisVal`) (`/Game/Blueprint/TankPawns/BP_PlayerTankBase.speed` _playertank)))))))

(fn `GetCurrentWeaponData`
  (returns (cooldownPercentage :type "Float (double-precision)") (Name :type String) (Ammo :type Integer))
  (bind _playertank (`self.playerTank`))
  (bind (_canshoot _cooldown) (`/Game/Blueprint/TankPawns/BP_PlayerTankBase.GetCurrentCoolDown` _playertank))
  (bind (_weapontype _ammo) (`/Game/Blueprint/PlayerInterface.GetWeaponStats` _playertank))
  (return _cooldown (`|GetEnumeratorNameAsString` _weapontype) _ammo))

(fn `GetRayCastEssentials`
  (params (`Ray cast Range` :type "Float (single-precision)"))
  (returns (End :type "Vector Structure") (Start :type "Vector Structure"))
  (return (+ (`.world location` (`self.BarrelTipLoc/Rot`)) (* (`KismetMathLibrary.GetForwardVector` (`SceneComponent.K2_GetComponentRotation` (`self.BarrelTipLoc/Rot`))) (`KismetMathLibrary.Conv_DoubleToVector` `Ray cast Range`))) (`.world location` (`self.BarrelTipLoc/Rot`))))

(fn `GetTeam`
  (returns (Team :type "/Game/Blueprint/Teams/EnumTeams Enum"))
  (return (`self.Teams`)))

(fn `InitReferencePawn`
  (params (PlayerPawn :type "Pawn Object Reference"))
  (bind _output_get (set `self.PlayerPawn` PlayerPawn))
  ;[1 1 1] Cast to get BP class and set up components
  (bind _asbp_player_tank_base (cast `/Game/Blueprint/TankPawns/BP_PlayerTankBase` _output_get))
  (bind _output_get_2 (set `self.playerTank` _asbp_player_tank_base))
  (set `self.Body` (`/Game/Blueprint/TankPawns/BP_PlayerTankBase.Body` _output_get_2))
  (set `self.playerMovementCompo` (`Pawn.GetMovementComponent` (`self.PlayerPawn`))))

(fn `IsCoolDownComplete`
  (returns (canShoot :type Boolean) (coolDown :type "Float (double-precision)"))
  (bind (_canshoot _cooldown) (message `/Game/Blueprint/PlayerInterface.GetCurrentCoolDown` (`self.PlayerPawn`)))
  (return _canshoot _cooldown))

(fn `IsFiring`
  (returns (`Is Holding Fire` :type Boolean))
  (return (`self.isHoldingFire`)))

(fn `SetCurrentWeapon`
  (params (currentWeapon :type "/Game/Blueprint/Enums/EnumWeaponType Enum" :default "NewEnumerator4") (WeaponRef :type "/Game/Blueprint/WeaponPickUp/BP_PickUpBase Object Reference")))

(fn `UserConstructionScript`
  (`KismetArrayLibrary.Array_AddUnique` (`self.Actors to Ignore`) (`self.K2_GetPawn`)))