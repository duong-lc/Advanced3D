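; Base player controller for a tank game, handling movement, aiming, weapon firing and switching, team colors and lives.
; Axis input drives the movement component and timeline-lerps the body toward the input direction.
; The current weapon rotates in yaw toward a line trace deprojected from a UI cursor, with controls gated by a zombie-mode alive check.
; Death costs a life, then respawns through GM_Base using delayed re-possession, or removes the player.
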(event `self.ReceiveBeginPlay`
  ;[0.2266 0.427 1 1 50] Begin Play
  (`|ExecutionSequence`
    (:`then_0`
      (`self.InitReferencePawn` (`GameplayStatics.GetPlayerPawn` 0))
      (set `self.lives` (`KismetStringLibrary.Conv_StringToInt` (`GameplayStatics.ParseOption` (`GameModeBase.OptionsString` (`GameplayStatics.GetGameMode`)) "lives"))))))

(event `self.ReceiveTick`
  (params (DeltaSeconds :type "Float (single-precision)"))
  (bind (_returnvalue_x _returnvalue_y) (`KismetMathLibrary.BreakVector2D` (`WidgetLayoutLibrary.GetViewportSize`)))
  (bind _returnvalue_x_2 (`KismetMathLibrary.BreakVector2D` (`WidgetLayoutLibrary.GetViewportSize`)))
  (bind (_screenposition_x _screenposition_y) (`KismetMathLibrary.BreakVector2D` (`/Game/Blueprint/PlayerControllers/UI_MouseCursor.CursorPos` (`self.CursorUI`))))
  (bind (_worldlocation _worlddirection) (`self.DeprojectScreenPositionToWorld` (+ (/ _returnvalue_x_2 2.0) _screenposition_x) (+ (/ _returnvalue_y 2.0) _screenposition_y)))
  (bind _returnvalue (+ (+ (* (`self.GetActorForwardVector` (`self.PlayerPawn`)) (* (`self.fwdAxisVal`) 100.0)) (* (`self.GetActorRightVector` (`self.PlayerPawn`)) (* (`self.rightAxisVal`) 100.0))) (`self.K2_GetActorLocation` (`self.PlayerPawn`))))
  (bind (_returnvalue_roll _returnvalue_pitch _returnvalue_yaw) (`KismetMathLibrary.BreakRotator` (`KismetMathLibrary.FindLookAtRotation` (`SceneComponent.K2_GetComponentLocation` (`self.Body`)) _returnvalue)))
  (bind _returnvalue_2 (`KismetMathLibrary.MakeRotator` _returnvalue_roll 0.0 (+ _returnvalue_yaw 180.0)))
  ;[0.2699 0.4876 1 1 36] Tick
  (`/Engine/EditorBlueprintResources/StandardMacros.IsValid` (`self.PlayerPawn`)
    (:`Is Valid`
      (if (`self.CheckZombieModeAlive`)
        (`/Engine/EditorBlueprintResources/StandardMacros.IsValid` (`self.CursorUI`)
          (:`Is Valid`
            (`/Engine/EditorBlueprintResources/StandardMacros.IsValid` (`self.PlayerPawn`)
              (:`Is Valid`
                (`/Engine/EditorBlueprintResources/StandardMacros.IsValid` (`self.playerTank`)
                  (:`Is Valid`
                    (bind _weapontype (message `/Game/Blueprint/PlayerInterface.GetWeaponStats` (`self.PlayerPawn`)))
                    (bind _outhit (`KismetSystemLibrary.LineTraceSingle` _worldlocation (+ _worldlocation (* _worlddirection (`KismetMathLibrary.Conv_DoubleToVector` 10000.0))) "TraceTypeQuery2" false (`self.Actors to Ignore`)))
                    (bind (_weapon_ref _isfound) (`/Game/Blueprint/TankPawns/BP_PlayerTankBase.GetCurrentWeapon` (`self.playerTank`) _weapontype))
                    (if _isfound
                      (set `self.CursorWorldPos` (`.Location` (`GameplayStatics.BreakHitResult` _outhit)))
                      (bind (_returnvalue_roll_2 _returnvalue_pitch_2 _returnvalue_yaw_2) (`KismetMathLibrary.BreakRotator` (`KismetMathLibrary.FindLookAtRotation` (`self.K2_GetActorLocation` (`self.K2_GetPawn`)) (`.Location` (`GameplayStatics.BreakHitResult` _outhit)))))
                      (`SceneComponent.K2_SetWorldRotation` (`Actor.RootComponent` _weapon_ref) (`KismetMathLibrary.MakeRotator` 0.0 0.0 _returnvalue_yaw_2) false false)))))))))
      (`/Engine/EditorBlueprintResources/StandardMacros.IsValid` (`self.PlayerPawn`)
        (:`Is Valid`
          (`KismetSystemLibrary.DrawDebugLine` (`self.K2_GetActorLocation` (`self.PlayerPawn`)) _returnvalue (struct :`G` 1.0 :`B` 0.103821 :`A` 1.0) 0.0 1.0)
          ;;[1 1 1] If there's input, update the rotation
          (if (or (!= (`self.rightAxisVal`) 0.0) (!= (`self.fwdAxisVal`) 0.0))
            ;;[1 1 1] Check if it's the same rotator with tolerance
            (if (not (== _returnvalue_2 (`self.currBodyRotation`) :`ErrorTolerance` 0.1))
              (set `self.currBodyRotation` _returnvalue_2))))))))

(event `InputAxis|MoveRight`
  (params (AxisValue :type "Float (single-precision)"))
  (bind _body (`self.Body`))
  ;[1 0.1779 0.484 1 36] Movement
  (`/Engine/EditorBlueprintResources/StandardMacros.IsValid` (`self.PlayerPawn`)
    (:`Is Valid`
      (`/Engine/EditorBlueprintResources/StandardMacros.IsValid` (`self.playerMovementCompo`)
        (:`Is Valid`
          (if (`self.CheckZombieModeAlive`)
            (set `self.rightAxisVal` AxisValue)
            (`PawnMovementComponent.AddInputVector` (`self.playerMovementCompo`) (`self.Get RightVelocity`) false)
            (bind (_direction _alphalerp) (`Timeline|LerpRotation` :!via `PlayFromStart` :!label _label)
              (:`Update`
                (`/Engine/EditorBlueprintResources/StandardMacros.IsValid` _body
                  (:`Is Valid`
                    (`SceneComponent.K2_SetWorldRotation` _body (`KismetMathLibrary.RLerp` (`SceneComponent.K2_GetComponentRotation` (`self.Body`)) (`self.currBodyRotation`) _alphalerp true) false false)))))))))))

(event `InputAxis|MoveForward`
  (params (AxisValue :type "Float (single-precision)"))
  ;[1 0.1779 0.484 1 36] Movement
  (`/Engine/EditorBlueprintResources/StandardMacros.IsValid` (`self.PlayerPawn`)
    (:`Is Valid`
      (`/Engine/EditorBlueprintResources/StandardMacros.IsValid` (`self.playerMovementCompo`)
        (:`Is Valid`
          (if (`self.CheckZombieModeAlive`)
            (set `self.fwdAxisVal` AxisValue)
            (`PawnMovementComponent.AddInputVector` (`self.playerMovementCompo`) (`self.Get Fwd Velocity`) false)
            (goto _label :!via `PlayFromStart`)))))))

(event `InputAction|Fire`
  (params (Key :type "Key Structure"))
  (bind _playerpawn (`self.PlayerPawn`))
  ;[0.2819 0.7132 1 1 40] Combat
  (:`Pressed`
    (`/Engine/EditorBlueprintResources/StandardMacros.IsValid` (`self.PlayerPawn`)
      (:`Is Valid`
        (if (`self.CheckZombieModeAlive`)
          (bind _weapontype (message `/Game/Blueprint/PlayerInterface.GetWeaponStats` _playerpawn))
          (switch `/Game/Blueprint/Enums/EnumWeaponType` _weapontype
            (:`NewEnumerator0`
              (set `self.isHoldingFire` true)
              (`self.Fire` :!label _label_2))
            (:`NewEnumerator1`
              (`self.Fire`))
            (:`NewEnumerator2`
              (`self.Fire`))
            (:`NewEnumerator3`
              (`self.Fire`)))))))
  (:`Released`
    (`/Engine/EditorBlueprintResources/StandardMacros.IsValid` (`self.PlayerPawn`)
      (:`Is Valid`
        (if (`self.CheckZombieModeAlive`)
          (bind _weapontype_2 (message `/Game/Blueprint/PlayerInterface.GetWeaponStats` _playerpawn))
          (switch `/Game/Blueprint/Enums/EnumWeaponType` _weapontype_2
            (:`NewEnumerator0`
              (set `self.isHoldingFire` false)
              (goto _label_2))))))))

(event `SetAbility`
  (params (`new Ability` :type "/Game/Blueprint/Enums/EnumAbilityType Enum" :default "NewEnumerator0"))
  ;[1 0.9465 0.2199 1 40] Ability
  (`KismetSystemLibrary.DelayUntilNextTick`))

(event `InputAction|PrevWeapon`
  (params (Key :type "Key Structure"))
  ;[0.8325 0.2617 1 1 40] Weapon Slot
  ;;[1 1 1] Switch to Previous Slot
  (:`Pressed`
    (`/Engine/EditorBlueprintResources/StandardMacros.IsValid` (`self.PlayerPawn`)
      (:`Is Valid`
        (if (`self.CheckZombieModeAlive`)
          (message `/Game/Blueprint/PlayerInterface.ChangeToPrevWeapon` (`self.PlayerPawn`)))))))

(event `InputAction|NextWeapon`
  (params (Key :type "Key Structure"))
  ;[0.8325 0.2617 1 1 40] Weapon Slot
  ;;[1 1 1] Switch to Next Slot
  (:`Pressed`
    (`/Engine/EditorBlueprintResources/StandardMacros.IsValid` (`self.PlayerPawn`)
      (:`Is Valid`
        (if (`self.CheckZombieModeAlive`)
          (message `/Game/Blueprint/PlayerInterface.ChangeToNextWeapon` (`self.PlayerPawn`)))))))

(event `/Game/Blueprint/PlayerControllers/Interface_PC.OnWeaponChange`
  (set `self.isHoldingFire` false))

(event `self.ReceivePossess`
  (params (PossessedPawn :type "Pawn Object Reference"))
  (`self.InitReferencePawn` PossessedPawn)
  (`self.ResetAllStats`)
  ;[1 1 1] UnHide Actor
  (`/Game/Blueprint/TankPawns/BP_PlayerTankBase.UnhidePlayer` (`self.playerTank`))
  (switch `/Game/Blueprint/Teams/EnumTeams` (`self.Teams`)
    (:`NewEnumerator0`
      (`/Game/Blueprint/TankPawns/BP_PlayerTankBase.Set Body Color` (`self.playerTank`) "/Game/Assets/EnemyMesh/En_Mat02.En_Mat02"))
    (:`NewEnumerator1`
      (`/Game/Blueprint/TankPawns/BP_PlayerTankBase.Set Body Color` (`self.playerTank`) "/Game/Assets/EnemyMesh/En_Mat01.En_Mat01"))
    (:`NewEnumerator2`
      (`/Game/Blueprint/TankPawns/BP_PlayerTankBase.Set Body Color` (`self.playerTank`) "/Game/Assets/EnemyMesh/En_Mat01_2.En_Mat01_2"))))

(event `/Game/Blueprint/PlayerControllers/Interface_PC.PawnDied`
  (`KismetSystemLibrary.PrintString` "DEATH" true true (struct :`R` 0.697051 :`G` 0.033717 :`B` 1.0 :`A` 1.0))
  (bind _result (`/Engine/EditorBlueprintResources/StandardMacros.DecrementInt` (`self.lives`))
    (:`  `
      (if (>= _result 1)
        (`KismetSystemLibrary.Delay` 1.0)
        (`self.UnPossess` self)
        (bind _asgm_base (cast `/Game/Blueprint/GameModes/GM_Base` (`GameplayStatics.GetGameMode`)))
        (`/Game/Blueprint/GameModes/GM_Base.Spawn Player` _asgm_base self)
        (`KismetSystemLibrary.PrintString` "restart base" true true (struct :`R` 1.0 :`B` 0.68045 :`A` 1.0))
        (else
          (`GameplayStatics.RemovePlayer` self true))))))

(event `self.ReceiveUnPossess`
  (params (UnpossessedPawn :type "Pawn Object Reference"))
  (bind _new_pawn (`self.UnPossesses` UnpossessedPawn))
  ;[1 1 1] Respawn Delay
  (`KismetSystemLibrary.Delay` 3.0)
  (`/Engine/EditorBlueprintResources/StandardMacros.IsValid` _new_pawn
    (:`Is Valid`
      ;[1 1 1] Re-possess
      (`self.Possess` self _new_pawn))))

(event `InputAction|ReadyUp`
  (params (Key :type "Key Structure"))
  (:`Pressed`
    (set `self.isReady` (not (`self.isReady`)))))

(event `/Game/Blueprint/PlayerControllers/Interface_TeamPlayerController.SetTeam`
  (params (`Team to Set` :type "/Game/Blueprint/Teams/EnumTeams Enum" :default "NewEnumerator0"))
  (set `self.Teams` `Team to Set`))

(event `/Game/Blueprint/PlayerControllers/Interface_TeamPlayerController.SetPlayerStart`
  (params (SpawnPoint :type "/Game/Blueprint/Teams/BP_TankPlayerStart Object Reference"))
  (set `self.CurrentSpawner` SpawnPoint))

(fn `Ability_Activate`
  (params (Scale :type "Vector Structure") (maxHealth :type "Float (double-precision)") (speed :type "Float (double-precision)") (Material :type "MaterialInterface Object Reference"))
  (locals (mat :type "MaterialInterface Object Reference") (scaleToSet :type "Vector Structure") (maxHealthToSet :type "Float (double-precision)") (speedToSet :type "Float (double-precision)"))
  (`|ExecutionSequence`
    (:`then_0`
      (set `local.scaleToSet` Scale))
    (:`then_1`
      (set `local.maxHealthToSet` maxHealth))
    (:`then_2`
      (set `local.speedToSet` speed))
    (:`then_3`
      (set `local.mat` Material))
    (:`then_4`
      (`|ExecutionSequence`
        (:`then_0`
          ;[1 1 1] Set Tank Scale
          (`SceneComponent.SetWorldScale3D` (`/Game/Blueprint/TankPawns/BP_PlayerTankBase.Body` (`self.playerTank`)) (`local.scaleToSet`)))
        (:`then_1`
          ;[1 1 1] Set Health and max Health
          (bind _output_get (set `/Game/Blueprint/TankPawns/BP_PlayerTankBase.maxHealth` (`local.maxHealthToSet`) (`self.playerTank`)))
          (set `/Game/Blueprint/TankPawns/BP_PlayerTankBase.Health` _output_get (`self.playerTank`)))
        (:`then_2`
          ;[1 1 1] Set Speed
          (set `/Game/Blueprint/TankPawns/BP_PlayerTankBase.speed` (`local.speedToSet`) (`self.playerTank`)))
        (:`then_3`
          ;[1 1 1] Set Material
          (`PrimitiveComponent.SetMaterial` (`/Game/Blueprint/TankPawns/BP_PlayerTankBase.Body` (`self.playerTank`)) 0 (`local.mat`)))
        (:`then_4`
          (switch `/Game/Blueprint/Enums/EnumAbilityType` "NewEnumerator0"
            (:`NewEnumerator0`
              (`PrimitiveComponent.SetMaterial` (`/Game/Blueprint/TankPawns/BP_PlayerTankBase.Body` (`self.playerTank`)) 1 "/Game/Assets/EnemyMesh/En_Mat02.En_Mat02" :!label _label))
            (:`NewEnumerator1`
              (goto _label))
            (:`NewEnumerator2`
              (goto _label))
            (:`NewEnumerator3`
              (`PrimitiveComponent.SetMaterial` (`/Game/Blueprint/TankPawns/BP_PlayerTankBase.Body` (`self.playerTank`)) 1 "/Game/Assets/EnemyMesh/AlphaMat.AlphaMat"))))))))

(fn `AmmoDecrement`
  (returns (isSlotEmpty :type Boolean))
  (bind _weapontype (message `/Game/Blueprint/PlayerInterface.GetWeaponStats` (`self.PlayerPawn`)))
  ;[1 1 1] Removing an ammo count in inventory according to current weapon's enum.
  (bind _isslotempty (`/Game/Blueprint/InventorySystem/BP_InventoryComponent.RemoveItem` (`/Game/Blueprint/TankPawns/BP_PlayerTankBase.InventoryComponent` (`self.playerTank`)) _weapontype))
  ;[1 1 1] Check if current slot is empty
  (if _isslotempty
    ;[1 1 1] Getting next available slot in inventory
    (bind (_newcurrenum _newcurriventoryslot _canget) (`/Game/Blueprint/InventorySystem/BP_InventoryComponent.GetNextAvailable` (`/Game/Blueprint/TankPawns/BP_PlayerTankBase.InventoryComponent` (`self.playerTank`))))
    (`KismetSystemLibrary.PrintString` (`KismetStringLibrary.Concat_StrStr` (`|GetEnumeratorNameAsString` _newcurrenum) " weapon type lol"))
    ;[1 1 1] Check If "Next Available Slot" was able to get to, if it is, set that as current weapon, if not, then ignore getting and setting to next available slot
    (if _canget
      (message `/Game/Blueprint/PlayerInterface.ChangeToWeapon` (`self.playerTank`) _newcurrenum)))
  (return _isslotempty))

(fn `AmmoUsed`
  (returns (`is Slot Empty` :type Boolean))
  (bind _isslotempty (`self.AmmoDecrement`))
  (return _isslotempty))

(fn `CheckZombieModeAlive`
  (returns (canExecute :type Boolean))
  (bind (_iszombiemode _isequal) (message `/Game/Blueprint/PlayerControllers/Interface_PC_Zombie.IsAlive` self "NewEnumerator0"))
  (if _iszombiemode
    (if _isequal
      _
      (else
        _))
    (return _isequal)
    (else
      (return true))))

(fn `Fire`
  (bind _weapontype (message `/Game/Blueprint/PlayerInterface.GetWeaponStats` (`self.PlayerPawn`)))
  (bind (_weapon_ref _isfound) (`/Game/Blueprint/TankPawns/BP_PlayerTankBase.GetCurrentWeapon` (`self.playerTank`) _weapontype))
  (if _isfound
    (message `/Game/Blueprint/WeaponPickUp/Interface_Weapon.FireWeapon` _weapon_ref)
    (else
      (`KismetSystemLibrary.PrintString` "CANNOT FIRE WEAPON"))))

(fn `Get Fwd Velocity`
  (returns (`Local Forward Vector` :type "Vector Structure"))
  (bind _playertank (`self.playerTank`))
  (`/Engine/EditorBlueprintResources/StandardMacros.IsValid` _playertank
    (:`Is Valid`
      (return (* (`self.GetActorForwardVector` _playertank) (* (`self.fwdAxisVal`) (`/Game/Blueprint/TankPawns/BP_PlayerTankBase.speed` _playertank)))))))

(fn `Get RightVelocity`
  (returns (`Local Right Vector` :type "Vector Structure"))
  (bind _playertank (`self.playerTank`))
  (`/Engine/EditorBlueprintResources/StandardMacros.IsValid` _playertank
    (:`Is Valid`
      (return (* (`self.GetActorRightVector` _playertank) (* (`self.rightAxisVal`) (`/Game/Blueprint/TankPawns/BP_PlayerTankBase.speed` _playertank)))))))

(fn `GetCurrentWeaponData`
  (returns (cooldownPercentage :type "Float (double-precision)") (Name :type String) (Ammo :type Integer))
  (bind _playertank (`self.playerTank`))
  (`/Engine/EditorBlueprintResources/StandardMacros.IsValid` _playertank
    (:`Is Valid`
      (bind (_canshoot _cooldown) (`/Game/Blueprint/TankPawns/BP_PlayerTankBase.GetCurrentCoolDown` _playertank))
      (bind (_weapontype _ammo) (`/Game/Blueprint/PlayerInterface.GetWeaponStats` _playertank))
      (return _cooldown (`|GetEnumeratorNameAsString` _weapontype) _ammo))))

(fn `GetJoyXY`
  (returns (`X Axis` :type "Float (double-precision)") (`Y Axis` :type "Float (double-precision)") (Sens :type "Float (double-precision)"))
  (return (`self.GetInputAxisValue`) (`self.GetInputAxisValue`) (`self.Sens`)))

(fn `GetTeam`
  (returns (Team :type "/Game/Blueprint/Teams/EnumTeams Enum"))
  (return (`self.Teams`)))

(fn `InitReferencePawn`
  (params (PlayerPawn :type "Pawn Object Reference"))
  (bind _returnvalue (`Pawn.GetMovementComponent` (`self.PlayerPawn`)))
  (bind _output_get (set `self.PlayerPawn` PlayerPawn))
  ;[1 1 1] Cast to get BP class and set up components
  (bind _asbp_player_tank_base (cast `/Game/Blueprint/TankPawns/BP_PlayerTankBase` _output_get))
  (bind _output_get_2 (set `self.playerTank` _asbp_player_tank_base))
  (set `self.Body` (`/Game/Blueprint/TankPawns/BP_PlayerTankBase.Body` _output_get_2))
  (set `self.playerMovementCompo` _returnvalue)
  (if (`KismetSystemLibrary.IsValid` _returnvalue)
    _))

(fn `IsCoolDownComplete`
  (returns (canShoot :type Boolean) (coolDown :type "Float (double-precision)"))
  (bind (_canshoot _cooldown) (message `/Game/Blueprint/PlayerInterface.GetCurrentCoolDown` (`self.PlayerPawn`)))
  (return _canshoot _cooldown))

(fn `IsFiring`
  (returns (`Is Holding Fire` :type Boolean))
  (return (`self.isHoldingFire`)))

(fn `LookAt_NegX`
  (bind _returnvalue (- (`self.MouseX`) 5.0))
  (if true
    (bind _weapontype (message `/Game/Blueprint/PlayerInterface.GetWeaponStats` (`self.PlayerPawn`)))
    (if (`.IsFound` (`/Game/Blueprint/TankPawns/BP_PlayerTankBase.GetCurrentWeapon` (`self.playerTank`) _weapontype))
      (`self.SetMouseLocation` (`KismetMathLibrary.FTrunc` _returnvalue) (`KismetMathLibrary.FTrunc` (`self.MouseY`)))
      (set `self.MouseX` _returnvalue))))

(fn `LookAt_NegY`
  (bind _returnvalue (- (`self.MouseY`) -5.0))
  (if true
    (bind _weapontype (message `/Game/Blueprint/PlayerInterface.GetWeaponStats` (`self.PlayerPawn`)))
    (if (`.IsFound` (`/Game/Blueprint/TankPawns/BP_PlayerTankBase.GetCurrentWeapon` (`self.playerTank`) _weapontype))
      (`self.SetMouseLocation` (`KismetMathLibrary.FTrunc` (`self.MouseX`)) (`KismetMathLibrary.FTrunc` _returnvalue))
      (set `self.MouseY` _returnvalue))))

(fn `LookAt_PosX`
  (bind _returnvalue (- (`self.MouseX`) -5.0))
  (if true
    (bind _weapontype (message `/Game/Blueprint/PlayerInterface.GetWeaponStats` (`self.PlayerPawn`)))
    (if (`.IsFound` (`/Game/Blueprint/TankPawns/BP_PlayerTankBase.GetCurrentWeapon` (`self.playerTank`) _weapontype))
      (`self.SetMouseLocation` (`KismetMathLibrary.FTrunc` _returnvalue) (`KismetMathLibrary.FTrunc` (`self.MouseY`)))
      (set `self.MouseX` _returnvalue))))

(fn `LookAt_PosY`
  (bind _returnvalue (- (`self.MouseY`) 5.0))
  (if true
    (bind _weapontype (message `/Game/Blueprint/PlayerInterface.GetWeaponStats` (`self.PlayerPawn`)))
    (if (`.IsFound` (`/Game/Blueprint/TankPawns/BP_PlayerTankBase.GetCurrentWeapon` (`self.playerTank`) _weapontype))
      (`self.SetMouseLocation` (`KismetMathLibrary.FTrunc` (`self.MouseX`)) (`KismetMathLibrary.FTrunc` _returnvalue))
      (set `self.MouseY` _returnvalue))))

(fn `LookAt_X`
  (params (X :type "Float (double-precision)"))
  (bind _returnvalue (+ (`self.MouseX`) (* X 5.0)))
  (if true
    (bind _weapontype (message `/Game/Blueprint/PlayerInterface.GetWeaponStats` (`self.PlayerPawn`)))
    (if (`.IsFound` (`/Game/Blueprint/TankPawns/BP_PlayerTankBase.GetCurrentWeapon` (`self.playerTank`) _weapontype))
      (`self.SetMouseLocation` (`KismetMathLibrary.FTrunc` _returnvalue) (`KismetMathLibrary.FTrunc` (`self.MouseY`)))
      (set `self.MouseX` _returnvalue))))

(fn `ResetAllStats`
  (bind _playertank (`self.playerTank`))
  (set `/Game/Blueprint/TankPawns/BP_PlayerTankBase.Health` (`/Game/Blueprint/TankPawns/BP_PlayerTankBase.maxHealth` _playertank) _playertank))

(fn `UnPossesses`
  (params (pawnToUnPossess :type "Pawn Object Reference"))
  (returns (`new pawn` :type "Pawn Object Reference"))
  (locals (PawnToSet :type "Pawn Object Reference"))
  (`/Engine/EditorBlueprintResources/StandardMacros.IsValid` (`self.CurrentSpawner`)
    (:`Is Valid`
      ;[1 1 1] Set location
      (`self.K2_SetActorLocation` pawnToUnPossess (`self.K2_GetActorLocation` (`self.CurrentSpawner`)) false true)
      ;[1 1 1] Hide Actor
      (`/Game/Blueprint/TankPawns/BP_PlayerTankBase.HidePlayer` (`self.playerTank`))
      (bind _output_get (set `local.PawnToSet` pawnToUnPossess))
      (set `self.PlayerPawn` null)
      (set `self.playerTank` null)
      (return _output_get))
    (:`Is Not Valid`
      (`KismetSystemLibrary.PrintString` "SPAWNER NOT VALID")
      (return null))))

(fn `UserConstructionScript`
  (`KismetArrayLibrary.Array_AddUnique` (`self.Actors to Ignore`) (`self.K2_GetPawn`)))