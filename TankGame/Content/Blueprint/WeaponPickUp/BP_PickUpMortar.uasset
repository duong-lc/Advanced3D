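; Mortar weapon pickup that sets its turret mesh and weapon type on top of a parent pickup's setup.
; On fire, it checks the owner's cooldown and an ammo check, then spawns a mortar round at the barrel tip socket.
; The round receives that start point, the owning player's cursor hit location as its target, and the damage value, then cooldown begins.
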(event `/Game/Blueprint/WeaponPickUp/Interface_Weapon.FireWeapon`
  ;[1 1 1 1 24] If not on cool down, shoot raycast, and spawn mortar actor
  (bind _canshoot (message `/Game/Blueprint/PlayerInterface.GetCurrentCoolDown` (`self.P_Owner`)))
  (if _canshoot
    (bind _is_slot_empty (`self.AmmoUsed`))
    (if (not _is_slot_empty)
      (bind (_start_pos _end_pos) (`self.GetRayCastData`))
      (bind _returnvalue (`|SpawnActorFromClass` "/Game/Blueprint/Projectiles/BP_MortarRound.BP_MortarRound_C" (`KismetMathLibrary.MakeTransform` _start_pos) "Undefined" "OverrideRootScale" null null))
      ;[1 1 1 1 24] Set Properties for mortar actor on spawn
      (`/Game/Blueprint/Projectiles/BP_MortarRound.OnSpawn` _returnvalue _start_pos _end_pos)
      (`/Game/Blueprint/Projectiles/BP_MortarRound.SetDamage` _returnvalue (`self.Damage`))
      (`self.InitiateCoolDown`))))

(fn `GetRayCastData`
  (returns (`Start Pos` :type "Vector Structure") (`End Pos` :type "Vector Structure"))
  (locals (ControllerIndex :type Integer) (startLocation :type "Vector Structure") (endLocation :type "Vector Structure"))
  (bind (_index _is_pc_found) (message `/Game/Blueprint/GameModes/Interface_GM.GetPlayerControllerIndex` (`GameplayStatics.GetGameMode`) (`self.P_Owner`)))
  (if _is_pc_found
    (bind _output_get (set `local.startLocation` (`SceneComponent.GetSocketLocation` (`self.PickUp`) "barrelTip")))
    (bind _output_get_2 (set `local.endLocation` (`.Location` (`GameplayStatics.BreakHitResult` (`PlayerController.GetHitResultUnderCursorByChannel` (`GameplayStatics.GetPlayerController` _index) "TraceTypeQuery1" true)))))
    (return _output_get _output_get_2)
    (else
      (`KismetSystemLibrary.PrintString` "Player Controller Not FOUND: BP_PICKUPNMORTAR" true true (struct :`R` 1.0 :`B` 0.039221 :`A` 1.0)))))

(fn `UserConstructionScript`
  (`parent.UserConstructionScript`)
  (`self.SetPickUpMesh` "/Game/Assets/EnemyMesh/EnemyTurret_G005.EnemyTurret_G005")
  (`self.SetWeaponType` "NewEnumerator2"))