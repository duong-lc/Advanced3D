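; BP_PickUpProjectile is a weapon pickup that uses the EnemyTurret_G001 mesh and fires projectiles for its owner.
; FireWeapon checks the owner's cooldown and the AmmoUsed result, then spawns a BP_TankBullet at the barrelTip socket.
; It sets the bullet's controller and damage, launches it via BulletTraverse and starts the cooldown.
; The construction script sets mesh and weapon type, while GetTurretData returns only zero vectors.
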(event `/Game/Blueprint/WeaponPickUp/Interface_Weapon.FireWeapon`
  (bind _pickup (`self.PickUp`))
  (bind _canshoot (message `/Game/Blueprint/PlayerInterface.GetCurrentCoolDown` (`self.P_Owner`)))
  (if _canshoot
    (bind _is_slot_empty (`self.AmmoUsed`))
    (if (not _is_slot_empty)
      (bind _returnvalue (`|SpawnActorFromClass` "/Game/Blueprint/Projectiles/BP_TankBullet.BP_TankBullet_C" (`KismetMathLibrary.MakeTransform` (`SceneComponent.GetSocketLocation` _pickup "barrelTip") (`SceneComponent.K2_GetComponentRotation` _pickup)) "Undefined" "OverrideRootScale" null null))
      (`/Engine/EditorBlueprintResources/StandardMacros.IsValid` _returnvalue
        (:`Is Valid`
          (set `/Game/Blueprint/Projectiles/BP_ProjectileBase.OwnerController` (`Pawn.GetController` (`self.P_Owner`)) _returnvalue)
          (set `/Game/Blueprint/Projectiles/BP_TankBullet.damage` 25.0 _returnvalue)
          (`/Game/Blueprint/Projectiles/BP_TankBullet.BulletTraverse` _returnvalue (* 30000.0 30.0))
          (`self.InitiateCoolDown`))))
    (else
      (`KismetSystemLibrary.PrintString` "can't shoot"))))

(fn `GetTurretData`
  (returns (`World Location` :type "Vector Structure") (`World Rotation` :type "Rotator Structure"))
  (return (0.0 0.0 0.0)))

(fn `UserConstructionScript`
  (`parent.UserConstructionScript`)
  (`self.SetPickUpMesh` "/Game/Assets/EnemyMesh/EnemyTurret_G001.EnemyTurret_G001")
  (`self.SetWeaponType` "NewEnumerator1"))