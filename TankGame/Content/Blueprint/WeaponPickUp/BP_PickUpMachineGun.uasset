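; Machine gun weapon pickup that sets its turret mesh and weapon type on construction and fires hitscan shots.
; FireWeapon starts cooldown, uses ammo and line-traces forward from the barrelTip socket, applying damage and spawning muzzle and impact particles.
; While the owner's controller reports fire held, it repeats shots whenever the owner's cooldown allows, polling on next-tick delays between shots.
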(event `self.FireWeapon`
  (bind _is_holding_fire (`self.IsHoldingFire`))
  (if _is_holding_fire :!label _label
    (`self.InitiateCoolDown`)
    (`self.AmmoUsed`)
    (bind _world_location (`self.GetTurretData`))
    (bind (_out_hit_impact_point _success_) (`self.FireRayCast` (`self.Range`) (`self.Damage`)))
    (if _success_
      (`GameplayStatics.SpawnEmitterAtLocation` "/Game/Assets/Particles/BasicMachineGunHitPAR.BasicMachineGunHitPAR" _out_hit_impact_point (`KismetMathLibrary.FindLookAtRotation` _world_location _out_hit_impact_point) (2.0 2.0 2.0)))
    (bind _is_holding_fire_2 (`self.IsHoldingFire` :!label _label_2))
    (if _is_holding_fire_2
      (bind _canshoot (message `/Game/Blueprint/PlayerInterface.GetCurrentCoolDown` (`self.P_Owner`)))
      (if _canshoot
        (goto _label)
        (else
          (`KismetSystemLibrary.DelayUntilNextTick`)
          (goto _label_2))))))

(fn `FireRayCast`
  (params (Range :type "Float (double-precision)") (Damage :type "Float (double-precision)"))
  (returns (`Out Hit Impact Point` :type "Vector Structure") (`Success?` :type Boolean))
  (bind (_start _end) (`self.GetRayCastData` Range))
  (`GameplayStatics.SpawnEmitterAtLocation` "/Game/Assets/Particles/BasicMachineGunFirePAR.BasicMachineGunFirePAR" _start (`KismetMathLibrary.FindLookAtRotation` _start _end) (1.5 1.5 1.5))
  (bind (_outhit _returnvalue) (`KismetSystemLibrary.LineTraceSingle` _start _end "TraceTypeQuery1"))
  (`GameplayStatics.ApplyDamage` (`.HitActor` (`GameplayStatics.BreakHitResult` _outhit)) Damage)
  (return (`.ImpactPoint` (`GameplayStatics.BreakHitResult` _outhit)) _returnvalue))

(fn `GetRayCastData`
  (params (`Ray cast Range` :type "Float (single-precision)"))
  (returns (Start :type "Vector Structure") (End :type "Vector Structure"))
  (bind (_world_location _world_rotation) (`self.GetTurretData`))
  (return _world_location (+ _world_location (* (`KismetMathLibrary.GetForwardVector` _world_rotation) (`KismetMathLibrary.Conv_DoubleToVector` `Ray cast Range`)))))

(fn `GetTurretData`
  (returns (`World Location` :type "Vector Structure") (`World Rotation` :type "Rotator Structure"))
  (bind _pickup (`self.PickUp`))
  (return (`SceneComponent.GetSocketLocation` _pickup "barrelTip") (`SceneComponent.K2_GetComponentRotation` _pickup)))

(fn `UserConstructionScript`
  (`parent.UserConstructionScript`)
  (`self.SetPickUpMesh` "/Game/Assets/EnemyMesh/EnemyTurret_G001M2.EnemyTurret_G001M2")
  (`self.SetWeaponType` "NewEnumerator0"))