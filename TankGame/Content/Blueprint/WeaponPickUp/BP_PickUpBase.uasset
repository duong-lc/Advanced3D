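; Base weapon pickup actor that a player tank collects by overlapping its sphere, which stops the rotation, removes the trigger, records the owner and notifies the tank.
; Setting the weapon type assigns that type's ammo count, and enable/disable functions toggle visibility, overlaps and rotation.
; Helpers relay ammo-use messages to the owner's controller and cooldown messages to the tank.
; FireWeapon and GetTurretData are placeholders, empty or returning zeroed values.
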(event `self.Sphere.OnComponentBeginOverlap`
  (params (OverlappedComponent :type "PrimitiveComponent Object Reference") (OtherActor :type "Actor Object Reference") (OtherComp :type "PrimitiveComponent Object Reference") (OtherBodyIndex :type Integer) (bFromSweep :type Boolean) (SweepResult :type "HitResult Structure (by ref)"))
  (bind _asbp_player_tank_base (cast `/Game/Blueprint/TankPawns/BP_PlayerTankBase` OtherActor))
  (`ActorComponent.K2_DestroyComponent` (`self.RotatingMovement`))
  (`ActorComponent.K2_DestroyComponent` (`self.Sphere`))
  (set `self.P_Owner` _asbp_player_tank_base)
  (message `/Game/Blueprint/PlayerInterface.OnWeaponPickUp` _asbp_player_tank_base self))

(event `/Game/Blueprint/WeaponPickUp/Interface_Weapon.FireWeapon`)

(fn `AmmoUsed`
  (message `/Game/Blueprint/PlayerControllers/Interface_PC.AmmoUsed` (`Pawn.GetController` (`self.P_Owner`)))
  (return))

(fn `DisableActor`
  (`ActorComponent.K2_DestroyComponent` (`self.RotatingMovement`))
  (`SceneComponent.SetVisibility` (`self.PickUp`) false false)
  (`SceneComponent.SetVisibility` (`self.Sphere`) false false)
  (set `PrimitiveComponent.bGenerateOverlapEvents` false (`self.Sphere`)))

(fn `EnableActor`
  (`|AddComponentByClass` "/Script/Engine.RotatingMovementComponent")
  (`SceneComponent.SetVisibility` (`self.PickUp`) true false)
  (`SceneComponent.SetVisibility` (`self.Sphere`) true false)
  (set `PrimitiveComponent.bGenerateOverlapEvents` true (`self.Sphere`)))

(fn `GenerateWeaponAmmo`
  (switch `/Game/Blueprint/Enums/EnumWeaponType` (`self.WeaponType`)
    (:`NewEnumerator0`
      (set `self.WeaponAmmo` 10))
    (:`NewEnumerator1`
      (set `self.WeaponAmmo` 30))
    (:`NewEnumerator2`
      (set `self.WeaponAmmo` 10))
    (:`NewEnumerator3`
      (set `self.WeaponAmmo` 5))))

(fn `Get Picked Up Weapon Ammo`
  (returns (WeaponAmmo :type Integer))
  (return (`self.WeaponAmmo`)))

(fn `GetPickUpMesh`
  (returns (`Static Mesh` :type "StaticMesh Object Reference"))
  (return (`StaticMeshComponent.StaticMesh` (`self.PickUp`))))

(fn `GetTurretData`
  (returns (`World Location` :type "Vector Structure") (`World Rotation` :type "Rotator Structure"))
  (return (0.0 0.0 0.0)))

(fn `InitiateCoolDown`
  (message `/Game/Blueprint/PlayerInterface.InitiateCurrentCoolDown` (`self.P_Owner`) (`self.WeaponType`))
  (return))

(fn `SetPickUpMesh`
  (params (NewMesh :type "StaticMesh Object Reference"))
  (`StaticMeshComponent.SetStaticMesh` (`self.PickUp`) NewMesh))

(fn `SetWeaponType`
  (params (WeaponType :type "/Game/Blueprint/Enums/EnumWeaponType Enum" :default "NewEnumerator0"))
  (set `self.WeaponType` WeaponType)
  (`self.GenerateWeaponAmmo`))

(fn `UserConstructionScript`)