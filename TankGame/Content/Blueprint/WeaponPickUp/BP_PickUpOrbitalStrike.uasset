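; Weapon pickup for an orbital strike that drops a rocket from the sky onto the player's cursor position.
; FireWeapon checks the owner's cooldown and the ammo state, spawns a BP_Rocket, sets its damage, sends it along its path and starts the cooldown.
; GetRayCastData takes the target from PC_Base's cursor world position and offsets the start point straight up, without performing a trace despite its name.
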(event `/Game/Blueprint/WeaponPickUp/Interface_Weapon.FireWeapon`
  ;[1 1 1 1 24] If not on cooldown, fire the rocket
  (bind _canshoot (message `/Game/Blueprint/PlayerInterface.GetCurrentCoolDown` (`self.P_Owner`)))
  (if _canshoot
    (bind _is_slot_empty (`self.AmmoUsed`))
    (if (not _is_slot_empty)
      (bind (_start_location _end_location) (`self.GetRayCastData`))
      (bind _returnvalue (`|SpawnActorFromClass` "/Game/Blueprint/Projectiles/BP_Rocket.BP_Rocket_C" (`KismetMathLibrary.MakeTransform` _start_location) "Undefined" "OverrideRootScale" null null :!pinned true)) ; Spawn Rocket blueprint actor
      ;[1 1 1 1 24] Setting properties of said spawned rocket
      (`/Game/Blueprint/Projectiles/BP_Rocket.SetDamage` _returnvalue 100.0)
      (`/Game/Blueprint/Projectiles/BP_Rocket.TraverseRocket` _returnvalue _start_location _end_location)
      (`self.InitiateCoolDown`))))

(fn `GetRayCastData`
  (returns (`Start Location` :type "Vector Structure") (`End Location` :type "Vector Structure"))
  (locals (endPos :type "Vector Structure") (startPos :type "Vector Structure"))
  (bind _returnvalue (`Pawn.GetController` (`self.P_Owner`)))
  (if (`KismetSystemLibrary.IsValid` _returnvalue)
    ;[1 1 1] Setting end position as the position of the mouse click into the world
    (bind _aspc_base (cast `/Game/Blueprint/PlayerControllers/PC_Base` _returnvalue))
    (bind _output_get (set `local.endPos` (`/Game/Blueprint/PlayerControllers/PC_Base.CursorWorldPos` _aspc_base)))
    ;[1 1 1] Start position is just end position with height offset
    (bind _output_get_2 (set `local.startPos` (+ _output_get (0.0 0.0 600.0))))
    (return _output_get_2 _output_get)
    (else
      (`KismetSystemLibrary.PrintString` "Player Controller Not FOUND: BP_PICKUPORBITALSTRIKE" true true (struct :`R` 1.0 :`B` 0.039221 :`A` 1.0)))))

(fn `UserConstructionScript`
  (`parent.UserConstructionScript`)
  (`self.SetPickUpMesh` "/Game/Assets/EnemyMesh/EnemyTurret_G006.EnemyTurret_G006")
  (`self.SetWeaponType` "NewEnumerator3"))