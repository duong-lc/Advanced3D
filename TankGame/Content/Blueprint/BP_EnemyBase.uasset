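; Base enemy Blueprint that tracks health and signals its own death.
; The Construction Script sets starting health from the enemy type (base, small or big).
; Any damage received feeds LoseHealth, which subtracts it, or clamps health to zero and calls EventEnemyDeath with itself when the hit is lethal.
; Each hit also prints the damage and remaining health as debug text.
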(event `self.ReceiveAnyDamage`
  (params (Damage :type "Float (single-precision)") (DamageType :type "DamageType Object Reference") (InstigatedBy :type "Controller Object Reference") (DamageCauser :type "Actor Object Reference"))
  (`self.LoseHealth` Damage))

(fn `LoseHealth`
  (params (loseAmount :type "Float (double-precision)"))
  (bind _returnvalue (- (`self.currHealth`) loseAmount))
  (if (<= _returnvalue 0.0)
    (set `self.currHealth` 0.0)
    (`self.EventEnemyDeath` self)
    (else
      (set `self.currHealth` _returnvalue)))
  (`KismetSystemLibrary.PrintString` (`KismetStringLibrary.Concat_StrStr` "Lose: " (`KismetStringLibrary.Conv_DoubleToString` loseAmount) " Remain: " (`KismetStringLibrary.Conv_DoubleToString` (`self.currHealth`)))))

(fn `UserConstructionScript`
  (switch `/Game/Blueprint/Enums/EnumEnemyType` (`self.enemyType`)
    (:`NewEnumerator0`
      (set `self.currHealth` 100.0))
    (:`NewEnumerator1`
      (set `self.currHealth` 50.0))
    (:`NewEnumerator2`
      (set `self.currHealth` 150.0))))