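; BP_InventorySlot is an actor representing one inventory slot for a shootable item, holding a pickup mesh reference, an ammo count and a cooldown.
; AddItem and RemoveItem adjust the count, with RemoveItem returning true when the last item is used, and DeleteSlot destroys the actor.
; InitiateCoolDown blocks shooting, Tick counts down until CanShoot is restored, and GetCoolDownPercent reports the remaining fraction.
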(event `self.ReceiveTick`
  (params (DeltaSeconds :type "Float (single-precision)"))
  (if (not (`self.canShoot`))
    (bind _output_get (set `self.currCoolDownTime` (- (`self.currCoolDownTime`) DeltaSeconds)))
    (if (<= _output_get 0.0)
      (set `self.currCoolDownTime` 0.0)
      (set `self.canShoot` true))))

(fn `Add Item`
  (params (`Item/Ammo to Add` :type Integer))
  (set `self.ItemCount` (+ `Item/Ammo to Add` (`self.ItemCount`))))

(fn `DeleteSlot`
  (`self.K2_DestroyActor` self))

(fn `GetAmmo`
  (returns (ammo :type Integer))
  (return (`self.ItemCount`)))

(fn `GetCoolDownPercent`
  (returns (percent :type "Float (double-precision)"))
  (return (/ (`self.currCoolDownTime`) (`self.CoolDownTime`))))

(fn `InitializeSlot`
  (params (mesh :type "StaticMesh Object Reference") (cooldown :type "Float (double-precision)"))
  (set `self.PickUpMeshRef` mesh)
  (set `self.CoolDownTime` cooldown))

(fn `InitiateCoolDown`
  (set `self.canShoot` false)
  (set `self.currCoolDownTime` (`self.CoolDownTime`)))

(fn `RemoveItem`
  (returns (isItemSlotEmpty :type Boolean))
  (if (<= (`self.ItemCount`) 1)
    (`/Engine/EditorBlueprintResources/StandardMacros.DecrementInt` (`self.ItemCount`)
      (:`  `
        (return true)))
    (else
      (`/Engine/EditorBlueprintResources/StandardMacros.DecrementInt` (`self.ItemCount`)
        (:`  `
          (return false))))))

(fn `UserConstructionScript`)