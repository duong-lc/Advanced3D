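; Weapon inventory component that stores the owning pawn's picked-up weapons in a map from weapon type to BP_InventorySlot actor.
; Pickups add ammo to an existing slot or spawn and initialize a new one, and removal deletes a slot once it reports empty.
; Next and previous lookups cycle through map key order with wraparound, while shoot checks and cooldowns are delegated to each slot.
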(event `self.ReceiveBeginPlay`)

(fn `AddItem`
  (params (WeaponPickUp :type "/Game/Blueprint/WeaponPickUp/BP_PickUpBase Object Reference"))
  (locals (weaponType :type "/Game/Blueprint/Enums/EnumWeaponType Enum" :default "NewEnumerator0") (inventorySlot :type "/Game/Blueprint/InventorySystem/BP_InventorySlot Object Reference") (Weapon :type "/Game/Blueprint/WeaponPickUp/BP_PickUpBase Object Reference"))
  (bind (_value _returnvalue) (`BlueprintMapLibrary.Map_Find` (`self.InventoryDictionary`) (`local.weaponType`)))
  ;[1 1 1] Setting Local variable
  (bind _output_get (set `local.Weapon` WeaponPickUp))
  (set `local.weaponType` (`/Game/Blueprint/WeaponPickUp/BP_PickUpBase.WeaponType` _output_get))
  ;[1 1 1] Find the Slot relative to the enum
  (set `local.inventorySlot` _value)
  (if _returnvalue
    ;[1 1 1] If it exists, add ammo
    (`/Game/Blueprint/InventorySystem/BP_InventorySlot.Add Item` (`local.inventorySlot`) (`/Game/Blueprint/WeaponPickUp/BP_PickUpBase.Get Picked Up Weapon Ammo` (`local.Weapon`)))
    (else
      ;[1 1 1] Create a new slot
      (bind _returnvalue_2 (`self.GetPlayerPawn`)
        (:`then`
          (bind _returnvalue_3 (`|SpawnActorFromClass` "/Game/Blueprint/InventorySystem/BP_InventorySlot.BP_InventorySlot_C" (`Actor.GetTransform` _returnvalue_2) "Undefined" "OverrideRootScale" _returnvalue_2 null))
          (`BlueprintMapLibrary.Map_Add` (`self.InventoryDictionary`) (`local.weaponType`) _returnvalue_3)
          ;[1 1 1] Get the new slot
          (`/Game/Blueprint/InventorySystem/BP_InventorySlot.InitializeSlot` _returnvalue_3 (`local.Weapon`) (`self.GetCoolDown` (`local.weaponType`)))
          ;[1 1 1] Add Ammo
          (`/Game/Blueprint/InventorySystem/BP_InventorySlot.Add Item` _returnvalue_3 (`/Game/Blueprint/WeaponPickUp/BP_PickUpBase.Get Picked Up Weapon Ammo` (`local.Weapon`))))))))

(fn `CheckCanShoot`
  (params (currWeapon :type "/Game/Blueprint/Enums/EnumWeaponType Enum" :default "NewEnumerator4"))
  (returns (canShoot :type Boolean) (coolDownPercent :type "Float (double-precision)"))
  (bind (_value _returnvalue) (`BlueprintMapLibrary.Map_Find` (`self.InventoryDictionary`) currWeapon))
  (if _returnvalue
    (return (`/Game/Blueprint/InventorySystem/BP_InventorySlot.canShoot` _value) (`/Game/Blueprint/InventorySystem/BP_InventorySlot.GetCoolDownPercent` _value))))

(fn `Get Next Item`
  (params (currWeapon :type "/Game/Blueprint/Enums/EnumWeaponType Enum" :default "NewEnumerator4"))
  (returns (Slot :type "/Game/Blueprint/InventorySystem/BP_InventorySlot Object Reference") (`next Weapon Enum` :type "/Game/Blueprint/Enums/EnumWeaponType Enum (by ref)") (shouldCycle :type Boolean))
  (locals (CurrentWeapon :type "/Game/Blueprint/Enums/EnumWeaponType Enum" :default "NewEnumerator4") (CurrWeaponIndex :type Integer) (nextWeaponIndex :type Integer))
  ;[1 1 1] Check for the size of current inventory, if the size isn't alloed, return false to not switch weapon
  (if (> (`self.GetInventorySize`) 1)
    (bind _output_get (set `local.CurrentWeapon` currWeapon))
    ;[1 1 1] Check if current weapon is not none.
    (`self.CheckCurrentWeapon` _output_get
      (:`is Not None`
        ;[1 1 1] Getting the next weapon index in the dictionary, which is looping through the keys in dictionary and return the int index.
        (bind _index (`self.GetCurrentWeaponIndex` (`local.CurrentWeapon`)))
        (bind _output_get_2 (set `local.CurrWeaponIndex` _index))
        ;[1 1 1] Check if the next index exceed the dictionary max index count?
        (if (== (+ _output_get_2 1) (`self.GetInventorySize`))
          ;[1 1 1] If it is, get the first one
          (set `local.nextWeaponIndex` 0)
          (else
            (set `local.nextWeaponIndex` (+ (`local.CurrWeaponIndex`) 1))))
        ;[1 1 1] Get the inventory slot
        (bind _values (`BlueprintMapLibrary.Map_Values` (`self.InventoryDictionary`)))
        ;[1 1 1] Get the enum
        (bind _keys (`BlueprintMapLibrary.Map_Keys` (`self.InventoryDictionary`)))
        (return (`|GetArrayItem` _values (`local.nextWeaponIndex`)) (`|GetArrayItem` _keys (`local.nextWeaponIndex`)) true)))
    (else
      (return null "NewEnumerator4" false))))

(fn `Get Slot`
  (params (Weapon :type "/Game/Blueprint/Enums/EnumWeaponType Enum" :default "NewEnumerator4"))
  (returns (`inventory slot` :type "/Game/Blueprint/InventorySystem/BP_InventorySlot Object Reference") (`is Valid` :type Boolean))
  (bind (_value _returnvalue) (`BlueprintMapLibrary.Map_Find` (`self.InventoryDictionary`) Weapon))
  (`self.CheckCurrentWeapon` Weapon
    (:`is Not None`
      (if _returnvalue
        (return _value _returnvalue)))))

(fn `GetCurrentWeaponIndex`
  (params (CurrWeapon :type "/Game/Blueprint/Enums/EnumWeaponType Enum" :default "NewEnumerator4"))
  (returns (Index :type Integer))
  (locals (CurrWeaponIndex :type Integer))
  (bind _keys (`BlueprintMapLibrary.Map_Keys` (`self.InventoryDictionary`)))
  (for (_array_element _array_index) _keys
    (if (`|EnumEquality` CurrWeapon _array_element)
      (bind _output_get (set `local.CurrWeaponIndex` _array_index))
      (break)))
  (return _output_get))

(fn `GetInventorySize`
  (returns (size :type Integer))
  (return (`BlueprintMapLibrary.Map_Length` (`self.InventoryDictionary`))))

(fn `GetNextAvailable`
  (returns (newCurrEnum :type "/Game/Blueprint/Enums/EnumWeaponType Enum (by ref)") (newCurrIventorySlot :type "/Game/Blueprint/InventorySystem/BP_InventorySlot Object Reference") (canGet :type Boolean))
  ;[1 1 1] Check if inventory isn't empty, if it is, return false (not able to get next available)
  (if (`BlueprintMapLibrary.Map_IsNotEmpty` (`self.InventoryDictionary`))
    ;[1 1 1] For all the keys that's in the dictionary, get the first entry and its value (inventory slot)
    (bind _keys (`BlueprintMapLibrary.Map_Keys` (`self.InventoryDictionary`)))
    (bind _output (`|GetArrayItem` _keys))
    (bind (_value _returnvalue) (`BlueprintMapLibrary.Map_Find` (`self.InventoryDictionary`) _output))
    ;[1 1 1] If find sucuessfully, return that new enum, and inventory slot.
    (if _returnvalue
      (return _output _value true)
      (else
        (`KismetSystemLibrary.PrintString` "BP_InventoryComponent: can't find iventory slot")))
    (else
      (return "NewEnumerator4" null false))))

(fn `GetPreviousItem`
  (params (`curr Weapon` :type "/Game/Blueprint/Enums/EnumWeaponType Enum" :default "NewEnumerator4"))
  (returns (slot :type "/Game/Blueprint/InventorySystem/BP_InventorySlot Object Reference") (`Previous weapon enum` :type "/Game/Blueprint/Enums/EnumWeaponType Enum (by ref)") (shouldCycle :type Boolean))
  (locals (CurrentWeapon :type "/Game/Blueprint/Enums/EnumWeaponType Enum") (CurrWeaponIndex :type Integer) (previousWeaponIndex :type Integer))
  ;[1 1 1] Check if the size would allow to get previous slot
  (if (> (`self.GetInventorySize`) 1)
    (bind _output_get (set `local.CurrentWeapon` `curr Weapon`))
    ;[1 1 1] Check if Current Weapon isn't none
    (`self.CheckCurrentWeapon` _output_get
      (:`is Not None`
        ;[1 1 1] Get Current Weapon Index
        (bind _index (`self.GetCurrentWeaponIndex` (`local.CurrentWeapon`)))
        (bind _output_get_2 (set `local.CurrWeaponIndex` _index))
        ;[1 1 1] Check if the previous slot goes below the first index of dictionary
        (if (< (- _output_get_2 1) 0)
          ;[1 1 1] If it is, return the last index in the dictionary
          (set `local.previousWeaponIndex` (- (`self.GetInventorySize`) 1))
          (else
            (set `local.previousWeaponIndex` (- (`local.CurrWeaponIndex`) 1))))
        ;[1 1 1] Get the Inventory Slot actor
        (bind _values (`BlueprintMapLibrary.Map_Values` (`self.InventoryDictionary`)))
        ;[1 1 1] Get the enum
        (bind _keys (`BlueprintMapLibrary.Map_Keys` (`self.InventoryDictionary`)))
        (return (`|GetArrayItem` _values (`local.previousWeaponIndex`)) (`|GetArrayItem` _keys (`local.previousWeaponIndex`)) true)))
    (else
      (return null "NewEnumerator4" false))))

(fn `GetSlotByType`
  (params (type :type "/Game/Blueprint/Enums/EnumWeaponType Enum" :default "NewEnumerator4"))
  (returns (Value :type "/Game/Blueprint/InventorySystem/BP_InventorySlot Object Reference") (IsFound :type Boolean))
  (locals (slot :type "/Game/Blueprint/InventorySystem/BP_InventorySlot Object Reference"))
  (bind (_value _returnvalue) (`BlueprintMapLibrary.Map_Find` (`self.InventoryDictionary`) type))
  (bind _output_get (set `local.slot` _value))
  (if _returnvalue
    (return _output_get _returnvalue)))

(fn `InitiateSlotCooldown`
  (params (currWeapon :type "/Game/Blueprint/Enums/EnumWeaponType Enum" :default "NewEnumerator4"))
  (bind (_value _returnvalue) (`BlueprintMapLibrary.Map_Find` (`self.InventoryDictionary`) currWeapon))
  (if _returnvalue
    (`/Game/Blueprint/InventorySystem/BP_InventorySlot.InitiateCoolDown` _value)))

(fn `RemoveItem`
  (params (WeaponType :type "/Game/Blueprint/Enums/EnumWeaponType Enum" :default "NewEnumerator0"))
  (returns (isSlotEmpty :type Boolean))
  (locals (typeToRemove :type "/Game/Blueprint/Enums/EnumWeaponType Enum" :default "NewEnumerator0") (inventorySlot :type "/Game/Blueprint/InventorySystem/BP_InventorySlot Object Reference"))
  (bind (_value _returnvalue) (`BlueprintMapLibrary.Map_Find` (`self.InventoryDictionary`) (`local.weaponType`)))
  (set `local.typeToRemove` WeaponType)
  ;[1 1 1] Getting the Slot based on the current weapon type
  (set `local.inventorySlot` _value)
  (if _returnvalue
    ;[1 1 1] Remove the Item slot (-- the item count), checks for if slot is empty
    (bind _isitemslotempty (`/Game/Blueprint/InventorySystem/BP_InventorySlot.RemoveItem` (`local.inventorySlot`)))
    (if _isitemslotempty
      ;[1 1 1] Destroy actor storing current slot's data, and remove key and value from dictionary
      (`/Game/Blueprint/InventorySystem/BP_InventorySlot.DeleteSlot` (`local.inventorySlot`))
      (bind _returnvalue_2 (`BlueprintMapLibrary.Map_Remove` (`self.InventoryDictionary`) (`local.typeToRemove`)))
      (`KismetSystemLibrary.PrintString` (`KismetStringLibrary.Concat_StrStr` "Remove  Item: " (`KismetStringLibrary.Conv_BoolToString` _returnvalue_2)))
      (return _returnvalue_2))))