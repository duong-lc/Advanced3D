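; PlayerDamageVolume is a zombie mode trigger volume that marks where player tanks should take damage.
; Its Box begin and end overlap events skip components tagged "ignoreZoneDmg" and cast the owning actor to P_TankZombieMode.
; Matching tanks are reported to the game mode through add and remove damage volume messages, so the volume applies no damage itself.
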(event `self.ReceiveActorBeginOverlap`
  (params (OtherActor :type "Actor Object Reference")))

(event `self.Box.OnComponentBeginOverlap`
  (params (OverlappedComponent :type "PrimitiveComponent Object Reference") (OtherActor :type "Actor Object Reference") (OtherComp :type "PrimitiveComponent Object Reference") (OtherBodyIndex :type Integer) (bFromSweep :type Boolean) (SweepResult :type "HitResult Structure (by ref)"))
  ;[1 1 1] Check for any objects that does not want to get damaged by the damage volume
  (if (not (`ActorComponent.ComponentHasTag` OtherComp "ignoreZoneDmg"))
    ;[1 1 1] Try casting to the player
    (bind _asp_tank_zombie_mode (cast `/Game/Blueprint/TankPawns/PlayerZombiePawns/P_TankZombieMode` (`ActorComponent.GetOwner` OtherComp)))
    ;[1 1 1] If it's a player that went to the damage volume, cause damage to them
    (message `/Game/Blueprint/GameModes/Interface_GM_Zombie.AddPlayerToDamageVolume` (`GameplayStatics.GetGameMode`) _asp_tank_zombie_mode)))

(event `self.Box.OnComponentEndOverlap`
  (params (OverlappedComponent :type "PrimitiveComponent Object Reference") (OtherActor :type "Actor Object Reference") (OtherComp :type "PrimitiveComponent Object Reference") (OtherBodyIndex :type Integer))
  ;[1 1 1] Check for any objects that does not want to get damaged by the damage volume
  (if (not (`ActorComponent.ComponentHasTag` OtherComp "ignoreZoneDmg"))
    ;[1 1 1] Try casting to the player
    (bind _asp_tank_zombie_mode (cast `/Game/Blueprint/TankPawns/PlayerZombiePawns/P_TankZombieMode` (`ActorComponent.GetOwner` OtherComp)))
    ;[1 1 1] If it's a player that went to the damage volume, cause damage to them
    (message `/Game/Blueprint/GameModes/Interface_GM_Zombie.RemovePlayerFromDamageVolume` (`GameplayStatics.GetGameMode`) _asp_tank_zombie_mode)))

(fn `UserConstructionScript`)