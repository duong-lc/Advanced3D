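; Zombie-mode spawner actor that spawns a given wave's enemies at random XY points inside its box, at the actor's height.
; SpawnZombies reads per-wave type and count entries, spawning each pawn with its mapped behavior tree and assigning its AI controller class afterward.
; It then passes its tracked zombie list to the game mode.
; Wave counts are stored by map Add, so GetEnemyCountInWave sees only the last recorded type's count.
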(event `self.ReceiveBeginPlay`
  (bind _asgm_zombie (cast `/Game/Blueprint/GameModes/GM_Zombie` (`GameplayStatics.GetGameMode`)))
  (set `self.CurrentGameMode` _asgm_zombie))

(fn `GetEnemyCountInWave`
  (params (wave :type Integer))
  (returns (EnemyCountInWave :type Integer))
  (locals (TotalEnemyInWave :type Integer))
  (bind _keys (`BlueprintMapLibrary.Map_Keys` (`self.WaveNumToEnemyCount`)))
  (for (_array_element _array_index) _keys
    (if (== wave _array_element)
      (bind _values (`BlueprintMapLibrary.Map_Values` (`self.WaveNumToEnemyCount`)))
      (set `local.TotalEnemyInWave` (+ (`|GetArrayItem` _values _array_index) (`local.TotalEnemyInWave`)))))
  (return (`local.TotalEnemyInWave`)))

(fn `GetRandomSpawnLoc`
  (returns (RandomLoc :type "Vector Structure"))
  (bind (_returnvalue_x _returnvalue_y _returnvalue_z) (`KismetMathLibrary.BreakVector` (`self.K2_GetActorLocation`)))
  (bind (_returnvalue_x_2 _returnvalue_y_2) (`KismetMathLibrary.BreakVector` (`BoxComponent.GetScaledBoxExtent` (`self.Box`))))
  (return (`KismetMathLibrary.MakeVector` (+ (`KismetMathLibrary.RandomFloatInRange` (* _returnvalue_x_2 -1.0) _returnvalue_x_2) _returnvalue_x) (+ _returnvalue_y (`KismetMathLibrary.RandomFloatInRange` (* _returnvalue_y_2 -1.0) _returnvalue_y_2)) _returnvalue_z)))

(fn `SpawnZombies`
  (params (`Curr Wave` :type Integer))
  (locals (CurrentWave :type Integer) (ZombiesInWaveList :type "Array of Pawn Object Reference"))
  (bind (_value _returnvalue) (`BlueprintMapLibrary.Map_Find` (`self.WaveData`) `Curr Wave`))
  (`KismetSystemLibrary.PrintString` "Start spawning")
  (set `local.CurrentWave` `Curr Wave`)
  ;[0.8652 0.2026 1] Getting Wave Data
  (if _returnvalue
    ;[0.1156 0.3649 1 1 12] For each Enemy Type In Wave Data
    (for _array_element (break `/Game/Blueprint/GameModes/Struct_ZombieDataSetPerWave` _value)
      (bind (_value_2 _returnvalue_2) (`BlueprintMapLibrary.Map_Find` (`self.ZombiePawn`) (break `/Game/Blueprint/GameModes/Struct_ZombieData` _array_element)))
      ;[0.1156 0.3649 1 1 12] Getting AI behavior tree
      (if _returnvalue_2
        ;[0.1156 0.3649 1 1 12] Track Total Enemy Count to Each Wave
        (`BlueprintMapLibrary.Map_Add` (`self.WaveNumToEnemyCount`) (`local.CurrentWave`) (`.SpawnCount_5_C62A7EE443596D84B94E6695F66B6403` (break `/Game/Blueprint/GameModes/Struct_ZombieData` _array_element)))
        ;[1 0.854 0.5852 1 12] For each Enemy To Spawn
        (for _ (range (`.SpawnCount_5_C62A7EE443596D84B94E6695F66B6403` (break `/Game/Blueprint/GameModes/Struct_ZombieData` _array_element)))
          ;[1 0.854 0.5852 1 12] Spawn Enemy
          (bind _returnvalue_3 (`AIBlueprintHelperLibrary.SpawnAIFromClass` (break `/Game/Blueprint/GameModes/Struct_ZombieData` _array_element) (`.AIBehaviorTreeBP_10_349D816846B3A7A44277518D78B76593` (break `/Game/Blueprint/ZombieModeSpecifics/SpawnerData` _value_2)) (`self.GetRandomSpawnLoc`) (struct) false null))
          ;[1 0.854 0.5852 1 12] Setting Zombie Pawns' Controller Class
          (`/Engine/EditorBlueprintResources/StandardMacros.IsValid` _returnvalue_3
            (:`Is Valid`
              (set `Pawn.AIControllerClass` (break `/Game/Blueprint/ZombieModeSpecifics/SpawnerData` _value_2) _returnvalue_3)
              ;[1 1 1] Track the enemy
              (`KismetArrayLibrary.Array_AddUnique` (`local.ZombiesInWaveList`) _returnvalue_3))))
        (else
          (`KismetSystemLibrary.PrintString` "Can't find Behavior tree in spawner"))))
    ;[1 1 1] All Enemies In Wave finished spawning
    (message `/Game/Blueprint/GameModes/Interface_GM.OnSpawnerCompleteSpawning` (`GameplayStatics.GetGameMode`) (`local.ZombiesInWaveList`))
    (`KismetSystemLibrary.PrintString` "Fin spawning")
    (else
      (`KismetSystemLibrary.PrintString` "Wave # not valid in spawner"))))

(fn `UserConstructionScript`)