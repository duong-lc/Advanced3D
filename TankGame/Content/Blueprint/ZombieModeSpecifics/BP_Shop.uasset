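; BP_Shop is a zombie-mode shop that sells a random pickup in exchange for a player's score.
; A sphere overlap tracks player controllers in range, found through the GetPCControllerMessage call on overlapping actors.
; SpawnRandomPickUp checks that the calling controller is in range and has enough Score, deducts the cost and spawns a random class at the spawn point, otherwise printing an insufficient-credits message.
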(event `self.Sphere.OnComponentBeginOverlap`
  (params (OverlappedComponent :type "PrimitiveComponent Object Reference") (OtherActor :type "Actor Object Reference") (OtherComp :type "PrimitiveComponent Object Reference") (OtherBodyIndex :type Integer) (bFromSweep :type Boolean) (SweepResult :type "HitResult Structure (by ref)"))
  (bind _pc_zombiemode (message `/Game/Blueprint/TankPawns/PlayerZombiePawns/Interface_PawnPlayerZombie.GetPC Controller` OtherActor))
  (if (!= _pc_zombiemode null)
    (`KismetArrayLibrary.Array_AddUnique` (`self.OverlapPCs`) _pc_zombiemode)))

(event `self.Sphere.OnComponentEndOverlap`
  (params (OverlappedComponent :type "PrimitiveComponent Object Reference") (OtherActor :type "Actor Object Reference") (OtherComp :type "PrimitiveComponent Object Reference") (OtherBodyIndex :type Integer))
  (bind _pc_zombiemode (message `/Game/Blueprint/TankPawns/PlayerZombiePawns/Interface_PawnPlayerZombie.GetPC Controller` OtherActor))
  (if (!= _pc_zombiemode null)
    (if (`KismetArrayLibrary.Array_Contains` (`self.OverlapPCs`) _pc_zombiemode)
      (`KismetArrayLibrary.Array_RemoveItem` (`self.OverlapPCs`) _pc_zombiemode))))

(fn `GetRandomPickUp`
  (returns (PickUpClass :type "/Game/Blueprint/WeaponPickUp/BP_PickUpBase Class Reference"))
  (return (`KismetArrayLibrary.Array_Random` (`self.PickUpClassToSpawn`))))

(fn `SpawnRandomPickUp`
  (params (`trigger PC` :type "/Game/Blueprint/PlayerControllers/PC_ZombieMode Object Reference"))
  (bind _returnvalue_location (`KismetMathLibrary.BreakTransform` (`SceneComponent.K2_GetComponentToWorld` (`self.SpawnPoint`))))
  ;[1 0.9985 0.4819] Checks if the PC calling is in range of the shop
  (if (`KismetArrayLibrary.Array_Contains` (`self.OverlapPCs`) `trigger PC`)
    ;[1 0.9985 0.4819] checking if enough score
    (if (>= (`/Game/Blueprint/PlayerControllers/PC_ZombieMode.Score` `trigger PC`) (`self.pointsToBuy`))
      ;[0.4033 1 0.5595] Decrementing score
      (set `/Game/Blueprint/PlayerControllers/PC_ZombieMode.Score` (- (`/Game/Blueprint/PlayerControllers/PC_ZombieMode.Score` `trigger PC`) (`self.pointsToBuy`)) `trigger PC`)
      ;[0.4107 0.9202 1] Spawn object
      (`|SpawnActorFromClass` (`self.GetRandomPickUp`) (`KismetMathLibrary.MakeTransform` _returnvalue_location) "Undefined" "OverrideRootScale" null null)
      (else
        (`KismetSystemLibrary.PrintString` "Insufficient credits" true true (struct :`R` 1.0 :`B` 0.003459 :`A` 1.0))))))

(fn `UserConstructionScript`)