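; BP_Door is a zombie-mode barrier that players buy open with score points.
; A Box trigger tracks overlapping players' PC controllers, obtained through GetPCControllerMessage on the overlapping actor, in the OverlapPCs array.
; OpenDoor accepts a triggering controller only if it is in that array, then deducts PointsToOpen from its Score and destroys the door, or prints an insufficient-credits message.
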(event `self.Box.OnComponentBeginOverlap`
  (params (OverlappedComponent :type "PrimitiveComponent Object Reference") (OtherActor :type "Actor Object Reference") (OtherComp :type "PrimitiveComponent Object Reference") (OtherBodyIndex :type Integer) (bFromSweep :type Boolean) (SweepResult :type "HitResult Structure (by ref)"))
  (bind _pc_zombiemode (message `/Game/Blueprint/TankPawns/PlayerZombiePawns/Interface_PawnPlayerZombie.GetPC Controller` OtherActor))
  (if (!= _pc_zombiemode null)
    (`KismetArrayLibrary.Array_AddUnique` (`self.Overlap PCs`) _pc_zombiemode)))

(event `self.Box.OnComponentEndOverlap`
  (params (OverlappedComponent :type "PrimitiveComponent Object Reference") (OtherActor :type "Actor Object Reference") (OtherComp :type "PrimitiveComponent Object Reference") (OtherBodyIndex :type Integer))
  (bind _pc_zombiemode (message `/Game/Blueprint/TankPawns/PlayerZombiePawns/Interface_PawnPlayerZombie.GetPC Controller` OtherActor))
  (if (!= _pc_zombiemode null)
    (if (`KismetArrayLibrary.Array_Contains` (`self.Overlap PCs`) _pc_zombiemode)
      (`KismetArrayLibrary.Array_RemoveItem` (`self.Overlap PCs`) _pc_zombiemode))))

(fn `OpenDoor`
  (params (TriggerPC :type "/Game/Blueprint/PlayerControllers/PC_ZombieMode Object Reference"))
  (if (`KismetArrayLibrary.Array_Contains` (`self.Overlap PCs`) TriggerPC)
    (if (>= (`/Game/Blueprint/PlayerControllers/PC_ZombieMode.Score` TriggerPC) (`self.PointsToOpen`))
      (set `/Game/Blueprint/PlayerControllers/PC_ZombieMode.Score` (- (`/Game/Blueprint/PlayerControllers/PC_ZombieMode.Score` TriggerPC) (`self.PointsToOpen`)) TriggerPC)
      (`self.K2_DestroyActor`)
      (else
        (`KismetSystemLibrary.PrintString` "Insufficient credits" true true (struct :`R` 1.0 :`B` 0.003459 :`A` 1.0))))))

(fn `UserConstructionScript`)