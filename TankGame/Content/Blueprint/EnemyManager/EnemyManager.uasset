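; EnemyManager tracks the living enemies in the level.
; On BeginPlay it gathers all BP_EnemyBase actors into an array and binds a handler to each one's enemy death event.
; The handler removes the dead enemy from the array and prints the remaining count.
; Only enemies present at BeginPlay are tracked, as nothing registers later spawns.
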(event `self.ReceiveBeginPlay`
  (bind _outactors (`GameplayStatics.GetAllActorsOfClass` "/Game/Blueprint/BP_EnemyBase.BP_EnemyBase_C"))
  (bind _output_get (set `self.EnemyArr` _outactors))
  (for _array_element _output_get
    (add `/Game/Blueprint/BP_EnemyBase.EventEnemyDeath` _array_element (`|CreateDelegate` :!event `CustomEvent_0`))))

(event `CustomEvent_0`
  (params (enemy :type "/Game/Blueprint/BP_EnemyBase Object Reference"))
  (bind _enemyarr (`self.EnemyArr`))
  (if (!= (`KismetArrayLibrary.Array_Find` _enemyarr enemy) -1)
    (bind _returnvalue (`KismetArrayLibrary.Array_RemoveItem` _enemyarr enemy))
    (if _returnvalue
      (`KismetSystemLibrary.PrintString` (`KismetStringLibrary.Concat_StrStr` "EnemyCount: " (`KismetStringLibrary.Conv_IntToString` (`KismetArrayLibrary.Array_Length` (`self.EnemyArr`))))))))

(fn `UserConstructionScript`)