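; Team-based spawn point for tanks that tracks which player controller is linked to it.
; The construction script sets a TextRender label and color from the Team enum: none, red or blue.
; LinkCurrentPCRef creates a two-way reference between spawner and controller, and IsOccupied checks that reference.
; Despite its name, IsOverlap returns true when the OverlapTanks array is empty; the event graph holds no active logic.
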(fn `IsOccupied`
  (returns (IsOccupied :type Boolean))
  (return (!= (`self.CurrentPCRef`) null)))

(fn `IsOverlap`
  (returns (canSpawn :type Boolean))
  (return (== (`KismetArrayLibrary.Array_Length` (`self.overlap tanks`)) 0)))

(fn `LinkCurrentPCRef`
  (params (CurrentPCRef :type "/Game/Blueprint/PlayerControllers/PC_Base Object Reference"))
  (returns (PCRef :type "/Game/Blueprint/PlayerControllers/PC_Base Object Reference"))
  (bind _output_get (set `self.CurrentPCRef` CurrentPCRef))
  (set `/Game/Blueprint/PlayerControllers/PC_Base.CurrentSpawner` self _output_get)
  (return _output_get))

(fn `UserConstructionScript`
  (switch `/Game/Blueprint/Teams/EnumTeams` (`self.Team`)
    (:`NewEnumerator0`
      (`TextRenderComponent.SetTextRenderColor` (`self.TextRender`) (`KismetMathLibrary.Conv_LinearColorToColor` (`KismetMathLibrary.LinearColor_White`)))
      (`TextRenderComponent.K2_SetText` (`self.TextRender`) (`|FormatText` "No Team")))
    (:`NewEnumerator1`
      (`TextRenderComponent.SetTextRenderColor` (`self.TextRender`) (`KismetMathLibrary.Conv_LinearColorToColor` (`KismetMathLibrary.LinearColor_Red`)))
      (`TextRenderComponent.K2_SetText` (`self.TextRender`) (`|FormatText` "Team Red")))
    (:`NewEnumerator2`
      (`TextRenderComponent.SetTextRenderColor` (`self.TextRender`) (`KismetMathLibrary.Conv_LinearColorToColor` (`KismetMathLibrary.LinearColor_Blue`)))
      (`TextRenderComponent.K2_SetText` (`self.TextRender`) (`|FormatText` "Team Blue")))))